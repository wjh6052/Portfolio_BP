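; Climbing component for BP_Player that attaches the character to walls and handles movement, corner turns and ledge climb-up.
; CheckClimbing switches to Flying and snaps the capsule to the wall after pelvis and head traces and a clearance check.
; ClimbingMove steers along the wall normal, triggering side turns when blocked, forward turns when the wall ends and climb-up when head height clears.
; Turns and climb-up play montages, some paired with MoveComponentTo.
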(event `self.ReceiveBeginPlay`
  (bind _asbp_player (cast `/Game/Player/BP_Player` (`self.GetOwner`)))
  (set `self.BP_Player` _asbp_player))

(event `CheckClimbing`
  (bind _bp_player (`self.BP_Player`))
  (bind _charactermovement (`Character.CharacterMovement` (`self.BP_Player`)))
  (bind _charactermovement_2 (`Character.CharacterMovement` _bp_player))
  (bind _head_hit (`self.Mid & Head Trace` 0.0)
    (:`then`
      (bind (_bblockinghit _binitialoverlap _time _distance _location _impactpoint _normal) (`GameplayStatics.BreakHitResult` _head_hit))
      ;[1 1 1] 올라탈 곳에 장애물 확인
      (bind (_outhit _returnvalue) (`KismetSystemLibrary.CapsuleTraceSingle` (`Actor.K2_GetActorLocation` (`self.GetOwner`)) (+ _location (* _normal 45.0)) 15.0 35.0 "TraceTypeQuery1")) ; 중간 캡슐 확인
      (if (not _returnvalue)
        ;[1 1 1] 클라이밍 선작업
        (`KismetSystemLibrary.Delay` 0.1)
        (`/Game/Interfaces/IState.SetMove` (`self.BP_Player`) false)
        (`/Game/Interfaces/IState.SetStatus` (`self.BP_Player`) "NewEnumerator1")
        (`CapsuleComponent.SetCapsuleRadius` (`Character.CapsuleComponent` (`self.BP_Player`)) 34.0 true)
        (`MovementComponent.StopMovementImmediately` _charactermovement)
        (`CharacterMovementComponent.SetMovementMode` _charactermovement "MOVE_Flying" 0)
        (set `CharacterMovementComponent.bOrientRotationToMovement` false _charactermovement_2)
        (set `CharacterMovementComponent.BrakingDecelerationFlying` (`CharacterMovementComponent.BrakingDecelerationWalking` _charactermovement_2) _charactermovement_2)
        (set `CharacterMovementComponent.MaxFlySpeed` 100.0 (`Character.CharacterMovement` (`self.BP_Player`)))
        (bind (_bblockinghit_2 _binitialoverlap_2 _time_2 _distance_2 _location_2 _impactpoint_2 _normal_2) (`GameplayStatics.BreakHitResult` _head_hit))
        (`KismetSystemLibrary.MoveComponentTo` (`Character.CapsuleComponent` (`self.BP_Player`)) (+ _location_2 (* _normal_2 (`CapsuleComponent.CapsuleRadius` (`Character.CapsuleComponent` _bp_player)))) (`KismetMathLibrary.Conv_VectorToRotator` (* _normal_2 -1.0)))
        (`/Game/Interfaces/IState.SetMove` (`self.BP_Player`) true)))))

(event `ClimbingMove_Up`
  (params (`Target Location` :type "Vector Structure"))
  (bind _returnvalue (+ `Target Location` (* (`Actor.GetActorForwardVector` (`self.BP_Player`)) 40.0)))
  ;[1 1 1] ClimbingMove_Up
  (bind (_outhit _returnvalue_2) (`KismetSystemLibrary.CapsuleTraceSingle` :`Start` `Target Location` :`End` _returnvalue :`Radius` 30.0 :`HalfHeight` (`CapsuleComponent.GetScaledCapsuleHalfHeight` (`Character.CapsuleComponent` (`self.BP_Player`))) :`TraceChannel` "TraceTypeQuery1" :`DrawDebugType` "ForDuration")) ; 올라갈 위치 확인
  (if (not _returnvalue_2)
    (`Character.PlayAnimMontage` (`self.BP_Player`) "/Game/Animation/Climbing/Turn/Climbing_Up_Top_Montage.Climbing_Up_Top_Montage" 1.0 "None")
    (`KismetSystemLibrary.Delay` 0.2)
    (`self.Climbing_End`)
    (`KismetSystemLibrary.MoveComponentTo` (`Character.CapsuleComponent` (`self.BP_Player`)) _returnvalue (`Actor.K2_GetActorRotation` (`self.BP_Player`)) false false 0.5)))

(event `ClimbingMove_SideTurn`
  (params (`Move Target` :type "Vector Structure") (`Axis Value` :type "Float (double-precision)"))
  (bind _bp_player (`self.BP_Player`))
  (bind _returnvalue (+ `Move Target` (* (`Actor.GetActorForwardVector` (`self.BP_Player`)) -60.0)))
  ;[1 1 1] ClimbingMove_SideTurn
  (bind (_outhit _returnvalue_2) (`KismetSystemLibrary.CapsuleTraceSingle` `Move Target` _returnvalue 29.0 35.0 "TraceTypeQuery1")) ; 옆쪽으로 체크
  (if (not _returnvalue_2)
    (bind (_outhit_2 _returnvalue_3) (`KismetSystemLibrary.LineTraceSingle` :`Start` _returnvalue :`End` (+ _returnvalue (* (`Actor.GetActorRightVector` (`self.BP_Player`)) (* `Axis Value` 100.0))) :`TraceChannel` "TraceTypeQuery1" :`DrawDebugType` "ForOneFrame")) ; 갈 방향 체크
    (if _returnvalue_3
      (if (> `Axis Value` 0.0)
        (`/Game/Interfaces/IState.SetMove` _bp_player false)
        (`Character.PlayAnimMontage` _bp_player "/Game/Animation/Climbing/Turn/Climbing_Turn_Side_R_Montage.Climbing_Turn_Side_R_Montage" 1.0 "None")
        (else
          (`/Game/Interfaces/IState.SetMove` _bp_player false)
          (`Character.PlayAnimMontage` _bp_player "/Game/Animation/Climbing/Turn/Climbing_Turn_Side_L_Montage.Climbing_Turn_Side_L_Montage" 1.0 "None")))
      (bind (_bblockinghit _binitialoverlap _time _distance _location _impactpoint _normal) (`GameplayStatics.BreakHitResult` _outhit_2))
      (`KismetSystemLibrary.MoveComponentTo` (`Character.CapsuleComponent` (`self.BP_Player`)) (+ _location (* _normal (`CapsuleComponent.CapsuleRadius` (`Character.CapsuleComponent` (`self.BP_Player`))))) (`KismetMathLibrary.Conv_VectorToRotator` (* _normal -1.0)) false false 0.7))))

(event `ClimbingMove_ForwradTurn`
  (params (`Move Target` :type "Vector Structure") (`Axis Value` :type "Float (double-precision)"))
  (bind _bp_player (`self.BP_Player`))
  (bind _returnvalue (+ `Move Target` (* (`Actor.GetActorRightVector` (`self.BP_Player`)) (* `Axis Value` 29.0))))
  ;[1 1 1] ClimbingMove_ForwradTurn
  (bind (_outhit _returnvalue_2) (`KismetSystemLibrary.CapsuleTraceSingle` :`Start` _returnvalue :`End` (+ _returnvalue (* (`Actor.GetActorForwardVector` (`self.BP_Player`)) 60.0)) :`Radius` 29.0 :`HalfHeight` 35.0 :`TraceChannel` "TraceTypeQuery1" :`DrawDebugType` "ForOneFrame")) ; 옆쪽으로 체크
  (if (not _returnvalue_2)
    (`/Game/Interfaces/IState.SetMove` (`self.BP_Player`) false)
    (if (> `Axis Value` 0.0)
      (`Character.PlayAnimMontage` _bp_player "/Game/Animation/Climbing/Turn/Climbing_Turn_Forwerd_R_Montage.Climbing_Turn_Forwerd_R_Montage" 1.0 "None")
      (else
        (`Character.PlayAnimMontage` _bp_player "/Game/Animation/Climbing/Turn/Climbing_Turn_Forwerd_L_Montage.Climbing_Turn_Forwerd_L_Montage" 1.0 "None")))))

(event `Climbing_End`
  (bind (_returnvalue_roll _returnvalue_pitch _returnvalue_yaw) (`KismetMathLibrary.BreakRotator` (`Actor.K2_GetActorRotation` (`self.BP_Player`))))
  (bind _charactermovement (`Character.CharacterMovement` (`self.BP_Player`)))
  ;[1 1 1] Climbing_End
  (`CharacterMovementComponent.SetMovementMode` (`Character.CharacterMovement` (`self.BP_Player`)) "MOVE_Falling" 0)
  (`CapsuleComponent.SetCapsuleRadius` (`Character.CapsuleComponent` (`self.BP_Player`)) 20.0 true)
  (set `CharacterMovementComponent.bOrientRotationToMovement` true _charactermovement)
  (set `CharacterMovementComponent.BrakingDecelerationFlying` 0.0 _charactermovement)
  (set `CharacterMovementComponent.MaxFlySpeed` 600.0 _charactermovement)
  (`/Game/Interfaces/IState.SetStatus` (`self.BP_Player`) "NewEnumerator0")
  (`Actor.K2_SetActorRotation` (`self.BP_Player`) (`KismetMathLibrary.MakeRotator` 0.0 (* _returnvalue_pitch 0.0) _returnvalue_yaw) false))

(fn `ClimbingMove`
  (params (`Dlrection Vector` :type "Vector Structure") (`Axis Value` :type "Float (double-precision)") (`On Side` :type Boolean))
  (locals (`Move Target` :type "Vector Structure"))
  (bind _returnvalue (`Actor.K2_GetActorLocation` (`self.BP_Player`)))
  (bind _returnvalue_2 (+ _returnvalue (* (`local.Dlrection Vector`) (* (`local.Axis Value`) 60.0))))
  (bind (_outhit _returnvalue_3) (`KismetSystemLibrary.CapsuleTraceSingle` :`Start` _returnvalue :`End` _returnvalue_2 :`Radius` 30.0 :`HalfHeight` 35.0 :`TraceChannel` "TraceTypeQuery1" :`DrawDebugType` "ForOneFrame")) ; 중간 캡슐 확인
  (if _returnvalue_3
    (set `local.Move Target` (`.Location` (`GameplayStatics.BreakHitResult` _outhit))) ; 헤드
    (if (`local.On Side`)
      (`self.ClimbingMove_SideTurn` (`local.Move Target`) (`local.Axis Value`))
      (else
        (bind (_head_hit _pelvis_hit _head) (`self.Mid & Head Trace` (`local.Axis Value`) (- (`local.Move Target`) (`Actor.K2_GetActorLocation` (`self.BP_Player`))) (`local.On Side`) :!label _label)
          (:`then`
            (bind (_bblockinghit _binitialoverlap _time _distance _location _impactpoint _normal) (`GameplayStatics.BreakHitResult` _pelvis_hit))
            (`Pawn.AddMovementInput` (`self.BP_Player`) (`KismetMathLibrary.GetDirectionUnitVector` (`Actor.K2_GetActorLocation` (`self.BP_Player`)) (+ _location (* _normal (`CapsuleComponent.CapsuleRadius` (`Character.CapsuleComponent` (`self.BP_Player`)))))) 1.0 false)
            (bind _returnvalue_4 (`KismetMathLibrary.RInterpTo` (`Actor.K2_GetActorRotation` (`self.BP_Player`)) (`KismetMathLibrary.Conv_VectorToRotator` (* _normal -1.0)) (`GameplayStatics.GetWorldDeltaSeconds`) 2.0))
            (`Actor.K2_SetActorRotation` (`self.BP_Player`) _returnvalue_4 false)
            (if (> (`KismetMathLibrary.Abs` (.pitch _returnvalue_4)) 60.0)
              (`self.Climbing_End`)))
          (:`No Head Block`
            (`self.ClimbingMove_Up` (+ _head (`KismetMathLibrary.MakeVector` 0.0 0.0 (`CapsuleComponent.GetScaledCapsuleHalfHeight` (`Character.CapsuleComponent` (`self.BP_Player`))))))))))
    (else
      (set `local.Move Target` _returnvalue_2) ; 허리
      (goto _label))))