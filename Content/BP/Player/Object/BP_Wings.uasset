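; BP_Wings is the player's wings actor, which shows or hides with a dissolve effect and animates wing flapping.
; Setting SpawnWings plays a timeline forward or in reverse on a dynamic dissolve material, then restores the wing material or hides the actor.
; A delayed timeline drives the WingL and WingR rotations.
; Sprinting stops and resets the flap and activates an attached Niagara trail; ending sprint reverses both.
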(event `self.ReceiveBeginPlay`
  (bind _skeletalmesh (`self.SkeletalMesh`))
  (bind _asbp_player (cast `/Game/BP/Player/BP_Player` (`self.GetOwner`)))
  (bind _output_get (set `self.BP_Player` _asbp_player))
  (set `self.BP Flight Component` (`/Game/BP/Player/BP_Player.BP_FlightComponent` _output_get))
  (bind _returnvalue (`NiagaraFunctionLibrary.SpawnSystemAttached` "/Game/Impact/FX/Niagara/System/Flight/NS_Wings_Trail.NS_Wings_Trail" (`self.SkeletalMesh`) "Center" (0.0 0.0 0.0) (struct :`Yaw` -90.0) "KeepRelativeOffset" false false))
  (set `self.Wings_Trail` _returnvalue)
  (bind _returnvalue_2 (`PrimitiveComponent.CreateDynamicMaterialInstance` _skeletalmesh 0 (`PrimitiveComponent.GetMaterial` _skeletalmesh 0) "None"))
  (set `self.Wings Dynamic Material` _returnvalue_2)
  (bind _returnvalue_3 (`KismetMaterialLibrary.CreateDynamicMaterialInstance` "/Game/Materials/MAT_Dissolve_Inst.MAT_Dissolve_Inst"))
  (set `self.DissolveMaterial` _returnvalue_3))

(event `Wings Move`
  (`KismetSystemLibrary.Delay` 1.0)
  (bind (_direction _out) (`Timeline|타임라인` :`NewTime` 0.5 :!via `PlayFromStart` :!label _label)
    (:`Update`
      (bind _returnvalue (* _out 70.0))
      (bind _returnvalue_2 (* _out 50.0))
      (set `self.Wing_L` (`KismetMathLibrary.MakeVector` 0.0 _returnvalue _returnvalue_2))
      (set `self.Wing_R` (`KismetMathLibrary.MakeVector` 0.0 _returnvalue _returnvalue_2)))))

(event `Wings Stop`
  (`|ExecutionSequence`
    (:`then_0`
      (goto _label :!via `Stop`))
    (:`then_1`
      (set `self.Wing_L` (0.0 0.0 0.0))
      (set `self.Wing_R` (0.0 0.0 0.0)))))

(event `Wings Start Sprint`
  (`self.Set Sprint` true))

(event `Spawn`
  (bind _spawntimelind (`self.SpawnTimelind`))
  (if (`self.bSpawn Wings`)
    (`self.SetActorHiddenInGame` false)
    (`PrimitiveComponent.SetMaterial` (`self.SkeletalMesh`) 0 (`self.DissolveMaterial`))
    (`TimelineComponent.SetPlayRate` _spawntimelind 1.5)
    (`self.Wings Move`)
    (bind (_direction _out_put) (`Timeline|SpawnTimelind` :!via `PlayFromStart` :!label _label_2)
      (:`Update`
        (`MaterialInstanceDynamic.SetScalarParameterValue` (`self.DissolveMaterial`) "Amount" _out_put))
      (:`Finished`
        (if (`self.bSpawn Wings`)
          (`PrimitiveComponent.SetMaterial` (`self.SkeletalMesh`) 0 (`self.Wings Dynamic Material`))
          (else
            (`self.SetActorHiddenInGame` (not (`self.bSpawn Wings`)))))))
    (else
      (`PrimitiveComponent.SetMaterial` (`self.SkeletalMesh`) 0 (`self.DissolveMaterial`))
      (`TimelineComponent.SetPlayRate` _spawntimelind 0.5)
      (goto _label_2 :!via `ReverseFromEnd`))))

(fn `Set Spawn Wings`
  (params (`In Spawn Wings` :type Boolean))
  (set `self.bSpawn Wings` `In Spawn Wings`)
  (`self.Spawn`))

(fn `Set Sprint`
  (params (`In Sprint` :type Boolean))
  (bind _output_get (set `self.bSprint` `In Sprint`))
  (`ActorComponent.SetActive` (`self.Wings_Trail`) _output_get _output_get)
  (if (`local.In Sprint`)
    (`self.Wings Stop`)
    (else
      (`self.Wings Move`))))

(fn `UserConstructionScript`)