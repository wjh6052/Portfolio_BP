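; Assassin melee decoration actor that attaches to the owning character's mesh at a data-asset socket and starts hidden.
; BeginPlay creates dynamic instances of its base material and a dissolve material.
; SpawnDecoration unhides the actor and plays a timeline driving the dissolve amount, then restores the base material.
; Despawning reapplies the dissolve material and reverses the timeline at a slower rate, without hiding the actor afterward.
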(event `self.ReceiveBeginPlay`
  (`parent.ReceiveBeginPlay`)
  (`self.K2_AttachToComponent` (`Character.Mesh` (`/Game/BP/Melee/BP_Melee.BP_Character` (`self.BP Melee`))) (`/Game/BP/Data/DataAsset/DABP_Melee.Decoration Socket Name` (`self.Owner Data Asset`)) "KeepRelative" "KeepRelative" "KeepRelative")
  (`self.SetActorHiddenInGame` true)
  (bind _returnvalue (`PrimitiveComponent.CreateDynamicMaterialInstance` (`self.SkeletalMesh`) 0 (`PrimitiveComponent.GetMaterial` (`self.SkeletalMesh`) 0) "None"))
  (set `self.Dynamic Material` _returnvalue)
  (bind _returnvalue_2 (`KismetMaterialLibrary.CreateDynamicMaterialInstance` "/Game/Materials/MAT_Dissolve_Inst.MAT_Dissolve_Inst"))
  (set `self.DissolveMaterial` _returnvalue_2))

(event `self.Spawn Decoration`
  (params (`In Spawn` :type Boolean))
  (bind _decoration_timeline (`self.Decoration_Timeline`))
  (bind _output_get (set `self.bSpawn` `In Spawn`))
  (if _output_get
    (`self.SetActorHiddenInGame` (not (`self.bSpawn`)))
    (`PrimitiveComponent.SetMaterial` (`self.SkeletalMesh`) 0 (`self.DissolveMaterial`))
    (`TimelineComponent.SetPlayRate` _decoration_timeline 1.5)
    (bind (_direction _out_put) (`Timeline|Decoration_Timeline` :!via `PlayFromStart` :!label _label)
      (:`Update`
        (`MaterialInstanceDynamic.SetScalarParameterValue` (`self.DissolveMaterial`) "Amount" _out_put))
      (:`Finished`
        (if (`self.bSpawn`)
          (`PrimitiveComponent.SetMaterial` (`self.SkeletalMesh`) 0 (`self.Dynamic Material`)))))
    (else
      (`PrimitiveComponent.SetMaterial` (`self.SkeletalMesh`) 0 (`self.DissolveMaterial`))
      (`self.SetActorHiddenInGame` (`self.bSpawn`))
      (`TimelineComponent.SetPlayRate` _decoration_timeline 0.5)
      (goto _label :!via `ReverseFromEnd`))))

(fn `UserConstructionScript`
  (`parent.UserConstructionScript`))