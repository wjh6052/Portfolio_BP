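; BP_Assassin is a melee weapon actor that attaches to the owning character's mesh at the equipment socket named in its data asset.
; On BeginPlay it creates dynamic instances of its own and a dissolve material, and resets Combo.
; SpawnWeapon swaps to the dissolve material and plays a timeline forward to appear, then restores the normal material, or in reverse to vanish and hide.
; Tick prints Combo for debugging.
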(event `self.ReceiveBeginPlay`
  (`parent.ReceiveBeginPlay`)
  (`self.K2_AttachToComponent` (`Character.Mesh` (`self.BP_Character`)) (`/Game/BP/Data/DataAsset/DABP_Melee.Equipment Socket Name` (`self.Data Asset`)) "KeepRelative" "KeepRelative" "KeepRelative")
  (bind _returnvalue (`PrimitiveComponent.CreateDynamicMaterialInstance` (`self.SkeletalMesh`) 0 (`PrimitiveComponent.GetMaterial` (`self.SkeletalMesh`) 0) "None"))
  (set `self.Dynamic Material` _returnvalue)
  (bind _returnvalue_2 (`KismetMaterialLibrary.CreateDynamicMaterialInstance` "/Game/Materials/MAT_Dissolve_Inst.MAT_Dissolve_Inst"))
  (set `self.DissolveMaterial` _returnvalue_2)
  (set `self.Combo` 0))

(event `self.Spawn Weapon`
  (params (`In Spawn` :type Boolean))
  (bind _bspawn (`self.bSpawn`))
  (bind _spawntimelind (`self.SpawnTimelind`))
  (bind _output_get (set `self.bSpawn` `In Spawn`))
  (if _output_get
    (`self.SetActorHiddenInGame` false)
    (`PrimitiveComponent.SetMaterial` (`self.SkeletalMesh`) 0 (`self.DissolveMaterial`))
    (`TimelineComponent.SetPlayRate` _spawntimelind 1.5)
    (bind (_direction _out_put) (`Timeline|SpawnTimelind` :!via `PlayFromStart` :!label _label)
      (:`Update`
        (`MaterialInstanceDynamic.SetScalarParameterValue` (`self.DissolveMaterial`) "Amount" _out_put))
      (:`Finished`
        (if _bspawn
          (`PrimitiveComponent.SetMaterial` (`self.SkeletalMesh`) 0 (`self.Dynamic Material`))
          (else
            (`self.SetActorHiddenInGame` (not _bspawn))))))
    (else
      (`PrimitiveComponent.SetMaterial` (`self.SkeletalMesh`) 0 (`self.DissolveMaterial`))
      (`TimelineComponent.SetPlayRate` _spawntimelind 0.5)
      (goto _label :!via `ReverseFromEnd`))))

(event `self.ReceiveTick`
  (params (DeltaSeconds :type "Float (single-precision)"))
  (`KismetSystemLibrary.PrintString` (`KismetStringLibrary.Conv_IntToString` (`self.Combo`)) true true (struct :`G` 0.66 :`B` 1.0 :`A` 1.0) 2.0 "5"))

(fn `UserConstructionScript`
  (`parent.UserConstructionScript`))