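; BP_Projectile is a short-lived projectile spawned by a BP_Melee owner to deliver hits on enemies.
; It caches its owner on BeginPlay and expires after a few seconds.
; SetActionData stores the combo, skill and jump-attack context of the triggering action.
; When its capsule overlaps a BP_Enemy, it disables collision, passes that context to the owner's HitOverlap flagged as a projectile hit, then destroys itself after a brief delay.
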(event `self.ReceiveBeginPlay`
  (bind _asbp_melee (cast `/Game/BP/Melee/BP_Melee` (`self.GetOwner`)))
  (set `self.BP Melee` _asbp_melee)
  (`self.SetLifeSpan` 3.0))

(event `self.Capsule.OnComponentBeginOverlap`
  (params (OverlappedComponent :type "PrimitiveComponent Object Reference") (OtherActor :type "Actor Object Reference") (OtherComp :type "PrimitiveComponent Object Reference") (OtherBodyIndex :type Integer) (bFromSweep :type Boolean) (SweepResult :type "HitResult Structure (by ref)"))
  (bind _asbp_enemy (cast `/Game/BP/Character/Enemy/BP_Enemy` OtherActor))
  (`PrimitiveComponent.SetCollisionEnabled` (`self.Capsule`) "NoCollision")
  (`/Game/BP/Melee/BP_Melee.Hit Overlap` (`self.BP Melee`) OverlappedComponent _asbp_enemy (`self.Combo Count`) (`self.Skill Count`) 0 (`self.In Jump Action`) false false true false)
  (`KismetSystemLibrary.Delay` 0.5)
  (`self.K2_DestroyActor`))

(fn `Set Action Data`
  (params (`In Combo Count` :type Integer) (`In Skill Count` :type Integer) (`In Jump Action` :type Boolean))
  (set `self.Combo Count` `In Combo Count`)
  (set `self.Skill Count` `In Skill Count`)
  (set `self.In Jump Action` `In Jump Action`))

(fn `UserConstructionScript`)