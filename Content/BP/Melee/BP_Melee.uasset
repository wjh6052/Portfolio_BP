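; Melee weapon actor owned by a BP_Character that handles equipping, combo attacks and toggling its hit capsule's collision.
; Equipping plays data asset montages, calls the empty SpawnWeapon event and swaps jump and rotation settings with unarmed values.
; Attack checks character status before playing the current combo montage, and queues a follow-up while the combo window is open.
; NextCombo consumes that queued input to advance through the data asset's action list, wrapping at the end.
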(event `self.ReceiveBeginPlay`
  (bind _asbp_character (cast `/Game/BP/Player/BP_Character` (`self.GetOwner`)))
  (set `self.BP_Character` _asbp_character))

(event `Spawn Weapon`
  (params (`In Spawn` :type Boolean)))

(fn `Attack`
  (bind _output_animmontage (break `/Game/BP/Data/DataAsset/DTS_ActionDatas` (`|GetArrayItem` (`/Game/BP/Data/DataAsset/DABP_Melee.Action Datas` (`self.Data Asset`)) (`self.Combo`))))
  (`self.Check Combo`)
  (if (or (`self.Check Status` "NewEnumerator0") (`self.Check Status` "NewEnumerator10"))
    (if (not (< (`self.Combo`) (`KismetArrayLibrary.Array_Length` (`/Game/BP/Data/DataAsset/DABP_Melee.Action Datas` (`self.Data Asset`)))))
      (set `self.Combo` 0))
    (for (_ _array_index) (`/Game/BP/Data/DataAsset/DABP_Melee.Action Datas` (`self.Data Asset`))
      (if (== _array_index (`self.Combo`))
        (`Character.PlayAnimMontage` (`self.BP_Character`) _output_animmontage 1.0 "None")
        (break)))
    (return)))

(fn `Can Combo`
  (params (`Can Combo` :type Boolean))
  (set `self.bCan Combo` `Can Combo`)
  (return))

(fn `Can Move`
  (params (`In Move` :type Boolean))
  (`/Game/BP/Interfaces/IState.SetMove` (`self.BP_Character`) `In Move`)
  (return))

(fn `Check Combo`
  (if (`self.bCan Combo`)
    (set `self.bNext Combo` true)))

(fn `Check Status`
  (params (StatusType :type "/Game/BP/Data/Enum/EStatusType Enum" :default "NewEnumerator0"))
  (returns (ReturnValue :type Boolean))
  (return (`|EnumEquality` (`/Game/BP/Player/BP_Character.StatusType` (`self.BP_Character`)) StatusType)))

(fn `Next Combo`
  (bind (_output_animmontage _output_power _output_playrate) (break `/Game/BP/Data/DataAsset/DTS_ActionDatas` (`|GetArrayItem` (`/Game/BP/Data/DataAsset/DABP_Melee.Action Datas` (`self.Data Asset`)) (`self.Combo`))))
  (if (`self.bNext Combo`)
    (set `self.Combo` (+ (`self.Combo`) 1))
    (set `self.bNext Combo` false)
    (if (not (< (`self.Combo`) (`KismetArrayLibrary.Array_Length` (`/Game/BP/Data/DataAsset/DABP_Melee.Action Datas` (`self.Data Asset`)))))
      (set `self.Combo` 0))
    (for (_ _array_index) (`/Game/BP/Data/DataAsset/DABP_Melee.Action Datas` (`self.Data Asset`))
      (if (== _array_index (`self.Combo`))
        (`Character.PlayAnimMontage` (`self.BP_Character`) _output_animmontage _output_playrate "None")
        (break)))
    (return)))

(fn `On Collision`
  (params (`On Collision` :type Boolean))
  (bind _capsule (`self.Capsule`))
  (if `On Collision`
    (`PrimitiveComponent.SetCollisionEnabled` _capsule "QueryAndPhysics")
    (else
      (`PrimitiveComponent.SetCollisionEnabled` _capsule "NoCollision"))))

(fn `Set Equip`
  (params (`In Equip` :type Boolean))
  (bind _data_asset (`self.Data Asset`))
  (if `In Equip`
    (`self.Set Move Data` true)
    (`self.Spawn Weapon` true)
    (`Character.PlayAnimMontage` (`self.BP_Character`) (`/Game/BP/Data/DataAsset/DABP_Melee.Equipment` _data_asset) 1.0 "None")
    (else
      (`self.Set Move Data` false)
      (`self.Spawn Weapon` false)
      (`Character.PlayAnimMontage` (`self.BP_Character`) (`/Game/BP/Data/DataAsset/DABP_Melee.UnEquipment` _data_asset) 1.0 "None"))))

(fn `Set Move Data`
  (params (`On Equip` :type Boolean))
  (bind (_move_value_jumpzvelocity _move_value_rotationrate) (break `/Game/BP/Data/DataAsset/DTS_MoveDatas` (`/Game/BP/Data/DataAsset/DABP_Melee.Move value` (`self.Data Asset`))))
  (bind _charactermovement (`Character.CharacterMovement` (`self.BP_Character`)))
  (bind (_move_value_jumpzvelocity_2 _move_value_rotationrate_2) (break `/Game/BP/Data/DataAsset/DTS_MoveDatas` (`/Game/BP/Data/DataAsset/DABP_Melee.Move value` (`self.DT_Unarmed`))))
  (bind _charactermovement_2 (`Character.CharacterMovement` (`self.BP_Character`)))
  (if `On Equip`
    (set `CharacterMovementComponent.JumpZVelocity` _move_value_jumpzvelocity _charactermovement)
    (set `CharacterMovementComponent.RotationRate` _move_value_rotationrate _charactermovement)
    (else
      (set `CharacterMovementComponent.JumpZVelocity` _move_value_jumpzvelocity_2 _charactermovement_2)
      (set `CharacterMovementComponent.RotationRate` _move_value_rotationrate_2 _charactermovement_2))))

(fn `UserConstructionScript`)