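; BP_Assassin is a player melee weapon actor that dissolves in and out when spawned or despawned.
; BeginPlay creates dynamic normal and dissolve materials, resets the combo count and disables weapon collision.
; SpawnWeapon swaps in the dissolve material and runs a timeline on its Amount parameter, faster forward for spawn and slower in reverse for despawn.
; The normal material returns after spawning, while despawning leaves the actor unhidden.
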(event `self.ReceiveBeginPlay`
  (`parent.ReceiveBeginPlay`)
  (bind _returnvalue (`PrimitiveComponent.CreateDynamicMaterialInstance` (`self.Weapon SkeletalMesh`) 0 (`PrimitiveComponent.GetMaterial` (`self.Weapon SkeletalMesh`) 0) "None"))
  (set `self.Dynamic Material` _returnvalue)
  (bind _returnvalue_2 (`KismetMaterialLibrary.CreateDynamicMaterialInstance` "/Game/Materials/MAT_Dissolve_Inst.MAT_Dissolve_Inst"))
  (set `self.DissolveMaterial` _returnvalue_2)
  (set `self.Combo Count` 0)
  (`PrimitiveComponent.SetCollisionEnabled` (`self.Weapon Collision`) "NoCollision"))

(event `self.Spawn Weapon`
  (params (`In Spawn` :type Boolean))
  (bind _spawntimelind (`self.SpawnTimelind`))
  (bind _output_get (set `self.bSpawn` `In Spawn`))
  (if _output_get
    (`self.SetActorHiddenInGame` (not (`self.bSpawn`)))
    (`PrimitiveComponent.SetMaterial` (`self.Weapon SkeletalMesh`) 0 (`self.DissolveMaterial`))
    (`TimelineComponent.SetPlayRate` _spawntimelind 1.5)
    (bind (_direction _out_put) (`Timeline|SpawnTimelind` :!via `PlayFromStart` :!label _label)
      (:`Update`
        (`MaterialInstanceDynamic.SetScalarParameterValue` (`self.DissolveMaterial`) "Amount" _out_put))
      (:`Finished`
        (if (`self.bSpawn`)
          (`PrimitiveComponent.SetMaterial` (`self.Weapon SkeletalMesh`) 0 (`self.Dynamic Material`)))))
    (else
      (`PrimitiveComponent.SetMaterial` (`self.Weapon SkeletalMesh`) 0 (`self.DissolveMaterial`))
      (`self.SetActorHiddenInGame` (`self.bSpawn`))
      (`TimelineComponent.SetPlayRate` _spawntimelind 0.5)
      (goto _label :!via `ReverseFromEnd`))))

(fn `UserConstructionScript`
  (`parent.UserConstructionScript`))