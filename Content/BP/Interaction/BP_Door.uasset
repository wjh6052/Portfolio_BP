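; BP_Door is an interactable swinging door that toggles open or closed each time a character interacts with it.
; BeginPlay sets up the Box as the Interact collision volume around the door.
; Interact flips Open and picks the swing sign from the dot product of door and character forward vectors, so the direction follows the character's facing.
; Tick eases the Door's rotation toward that yaw or back to zero with a constant-alpha lerp.
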(event `self.ReceiveBeginPlay`
  (`PrimitiveComponent.SetCollisionProfileName` (`self.Box`) "Interact" true)
  (`SceneComponent.K2_SetRelativeLocation` (`self.Box`) (0.0 0.0 105.0) false false)
  (`BoxComponent.SetBoxExtent` (`self.Box`) (25.0 60.0 110.0) true))

(event `self.ReceiveTick`
  (params (DeltaSeconds :type "Float (single-precision)"))
  (if (`self.bOpen`)
    (`SceneComponent.K2_SetRelativeRotation` (`self.Door`) (`KismetMathLibrary.RLerp` (`SceneComponent.RelativeRotation` (`self.Door`)) (`KismetMathLibrary.MakeRotator` 0.0 0.0 (`self.MaxYawWithDirection`)) (`self.ConstantRatio`)) false false)
    (else
      (`SceneComponent.K2_SetRelativeRotation` (`self.Door`) (`KismetMathLibrary.RLerp` (`SceneComponent.RelativeRotation` (`self.Door`)) (struct) (`self.ConstantRatio`)) false false))))

(fn `Interact`
  (params (InCharacter :type "/Game/BP/Character/BP_Character Object Reference"))
  (`parent.Interact` InCharacter)
  (set `self.MaxYawWithDirection` (* (`KismetMathLibrary.SignOfFloat` (`KismetMathLibrary.Dot_VectorVector` (`self.GetActorForwardVector`) (`self.GetActorForwardVector` InCharacter))) (`self.MaxYaw`)))
  (set `self.bOpen` (not (`self.bOpen`))))

(fn `UserConstructionScript`)