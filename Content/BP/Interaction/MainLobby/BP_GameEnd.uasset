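; BP_GameEnd is an interactable actor for the main lobby that quits the game.
; Its Box overlap registers it with an overlapping BP_MainLobby, passing its ObjectNameText, and leaving the box turns that interaction off and clears the text.
; Its Interact override calls the parent, then runs the Quit console command through player controller 0.
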(event `self.Box.OnComponentBeginOverlap`
  (params (OverlappedComponent :type "PrimitiveComponent Object Reference") (OtherActor :type "Actor Object Reference") (OtherComp :type "PrimitiveComponent Object Reference") (OtherBodyIndex :type Integer) (bFromSweep :type Boolean) (SweepResult :type "HitResult Structure (by ref)"))
  (bind _asbp_main_lobby (cast `/Game/BP/Character/BP_MainLobby` OtherActor))
  (`/Game/BP/Character/BP_MainLobby.Set Interaction` _asbp_main_lobby true self (`self.Object Name Text`)))

(event `self.Box.OnComponentEndOverlap`
  (params (OverlappedComponent :type "PrimitiveComponent Object Reference") (OtherActor :type "Actor Object Reference") (OtherComp :type "PrimitiveComponent Object Reference") (OtherBodyIndex :type Integer))
  (bind _asbp_main_lobby (cast `/Game/BP/Character/BP_MainLobby` OtherActor))
  (`/Game/BP/Character/BP_MainLobby.Set Interaction` _asbp_main_lobby false null ""))

(fn `Interact`
  (params (InCharacter :type "/Game/BP/Character/BP_Character Object Reference"))
  (`parent.Interact` InCharacter)
  (`KismetSystemLibrary.ExecuteConsoleCommand` "Quit" (`GameplayStatics.GetPlayerController` 0)))

(fn `UserConstructionScript`
  (`parent.UserConstructionScript`))