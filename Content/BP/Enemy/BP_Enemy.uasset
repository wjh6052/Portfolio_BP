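; BP_Enemy is a basic enemy Character that can be selected as a target and knocked back by attacks.
; On BeginPlay it shows its object name on a TextRender and starts deselected, with OnSelected and OnDeselected toggling the TargetWidget's visibility.
; AttackKnockBack launches it with the given vector, overriding current velocity.
; AnyDamage only prints the damage amount, with no health handling.
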(event `self.ReceiveBeginPlay`
  (`|ExecutionSequence`
    (:`then_0`
      (`TextRenderComponent.K2_SetText` (`self.TextRender`) (`KismetTextLibrary.Conv_StringToText` (`KismetSystemLibrary.GetObjectName` self))))
    (:`then_3`
      (`self.On Deselected`))))

(event `self.ReceiveAnyDamage`
  (params (Damage :type "Float (single-precision)") (DamageType :type "DamageType Object Reference") (InstigatedBy :type "Controller Object Reference") (DamageCauser :type "Actor Object Reference"))
  (`KismetSystemLibrary.PrintString` (`KismetStringLibrary.Conv_DoubleToString` Damage)))

(fn `Attack Knock Back`
  (params (`In Vector` :type "Vector Structure"))
  (`self.LaunchCharacter` `In Vector` true true))

(fn `On Deselected`
  (`SceneComponent.SetHiddenInGame` (`self.TargetWidget`) true false)
  (return))

(fn `On Selected`
  (`SceneComponent.SetHiddenInGame` (`self.TargetWidget`) false false))

(fn `UserConstructionScript`)