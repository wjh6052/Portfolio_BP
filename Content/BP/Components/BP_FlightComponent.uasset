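; Flight component for BP_Player that handles hovering, sprint flight, aiming and ground landing, switching movement mode, speeds, rotation, wings and montages.
; Tick derives lean from velocity-rotation deltas and updates a look-at point, while aiming adjusts the spring arm.
; Actor hits cancel sprint or, on flat ground with downward pitch, end flight through resettable DoOnce gates.
; Niagara effects pre-spawn inactive, with surface-based lookups; camera FOV eases through a zero-delay loop.
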(event `self.ReceiveBeginPlay`
  (bind _asbp_player (cast `/Game/BP/Character/BP_Player` (`self.GetOwner`)))
  (set `self.BP_Player` _asbp_player)
  (set `self.BP_CharacterMovement` (`Character.CharacterMovement` _asbp_player))
  (bind _returnvalue (`NiagaraFunctionLibrary.SpawnSystemAttached` (`self.Flight Trail`) (`Character.Mesh` (`self.BP_Player`)) "pelvis" (0.0 0.0 0.0) (struct :`Yaw` -90.0) "KeepRelativeOffset" false false))
  (set `self.Flight Trail Ref` _returnvalue)
  (bind _returnvalue_2 (`NiagaraFunctionLibrary.SpawnSystemAttached` (`self.FlightWave`) (`Actor.RootComponent` (`self.BP_Player`)) "None" (0.0 0.0 50.0) (struct :`Yaw` -90.0) "KeepRelativeOffset" false false))
  (set `self.FlightWaveRef` _returnvalue_2)
  (for (_array_element _array_index) (`self.FlightUnderDust`)
    (bind _returnvalue_3 (`NiagaraFunctionLibrary.SpawnSystemAttached` _array_element (`Actor.RootComponent` (`self.BP_Player`)) "None" (0.0 0.0 -150.0) (struct) "KeepRelativeOffset" false false))
    (`KismetArrayLibrary.Array_Insert` (`self.UnderDustRef`) _returnvalue_3 _array_index))
  (add `Actor.OnActorHit` (`self.BP_Player`) (delegate `hit`)))

(event `hit`
  (params (SelfActor :type "Actor Object Reference") (OtherActor :type "Actor Object Reference") (NormalImpulse :type "Vector Structure") (Hit :type "HitResult Structure (by ref)"))
  (bind (_returnvalue_roll _returnvalue_pitch _returnvalue_yaw) (`KismetMathLibrary.BreakRotator` (`Pawn.GetControlRotation` (`self.BP_Player`))))
  (bind (_returnvalue_roll_2 _returnvalue_pitch_2 _returnvalue_yaw_2) (`KismetMathLibrary.BreakRotator` (`Pawn.GetControlRotation` (`self.BP_Player`))))
  (bind (_returnvalue_roll_3 _returnvalue_pitch_3) (`KismetMathLibrary.BreakRotator` (`Pawn.GetControlRotation` (`self.BP_Player`))))
  (bind _returnvalue (`KismetMathLibrary.NormalizeToRange` _returnvalue_pitch_3 270.0 360.0))
  (bind _returnvalue_2 (> (.z (`.ImpactNormal` (`GameplayStatics.BreakHitResult` Hit))) 0.7))
  (if (`self.bFlying`)
    (if (`KismetMathLibrary.InRange_FloatFloat` _returnvalue 0.0 0.7)
      (if _returnvalue_2
        (if (`self.bSprint`)
          (if (< _returnvalue 0.65)
            (`/Engine/EditorBlueprintResources/StandardMacros.DoOnce` false :!label _label
              (:`Completed`
                (`self.StopFlight`)
                (`self.SetSprint` false)
                (set `self.bLanding` true)
                (`self.Stop To Play Anim` "/Game/Animation/Player/Flight/C_Landing_C_Montage.C_Landing_C_Montage")
                (set `self.bLanding` false)
                (`Controller.SetControlRotation` (`GameplayStatics.GetPlayerController` 0) (`KismetMathLibrary.MakeRotator` _returnvalue_roll 0.0 _returnvalue_yaw))))
            (else
              (`/Engine/EditorBlueprintResources/StandardMacros.DoOnce` false :!label _label_2
                (:`Completed`
                  (`self.StopFlight`)
                  (set `self.bLanding` true)
                  (`self.SetSprint` false)
                  (`self.Set Aiming` false)
                  (`Controller.SetControlRotation` (`GameplayStatics.GetPlayerController` 0) (`KismetMathLibrary.MakeRotator` _returnvalue_roll_2 0.0 _returnvalue_yaw_2))))))
          (else
            (goto _label_2)))
        (else
          (`self.SetSprint` false)))
      (elif (`self.bSprint`)
        (if (not _returnvalue_2)
          (`self.SetSprint` false))))))

(event `Hit Reset`
  (`|ExecutionSequence`
    (:`then_0`
      (goto _label :!via `Reset`))
    (:`then_1`
      (goto _label_2 :!via `Reset`))))

(event `StartFlight`
  (`/Game/BP/Character/BP_Character.Set State` (`self.BP_Player`) "NewEnumerator10")
  (`self.Set Flying` true)
  (`self.Set Flight Movement Param` true)
  (`/Game/BP/Character/BP_Player.Spawn Wings` (`self.BP_Player`) true)
  (`self.Stop To Play Anim` "/Game/Animation/Player/Flight/C_Flight_Hover_Start_C_Montage.C_Flight_Hover_Start_C_Montage")
  (set `CharacterMovementComponent.bOrientRotationToMovement` true (`Character.CharacterMovement` (`self.BP_Player`)))
  (`self.Hit Reset`))

(event `StopFlight`
  (bind _bp_player (`self.BP_Player`))
  (`/Game/BP/Character/BP_Player.EndSprint` _bp_player)
  (`/Game/BP/Character/BP_Character.Set State` _bp_player "NewEnumerator0")
  (`self.Set Flying` false)
  (`self.Set Flight Movement Param` false)
  (`self.Hit Reset`)
  (`/Game/BP/Character/BP_Player.Spawn Wings` (`self.BP_Player`) false)
  (`self.SetSprint` false))

(event `self.ReceiveTick`
  (params (DeltaSeconds :type "Float (single-precision)"))
  (bind _returnvalue (`GameplayStatics.GetWorldDeltaSeconds`))
  (bind _returnvalue_2 (`GameplayStatics.GetWorldDeltaSeconds`))
  (bind _lastvelocityrotation (`self.LastVelocityRotation`))
  (bind _bp_player (`self.BP_Player`))
  (bind _bp_player_2 (`self.BP_Player`))
  (bind (_lean_x _lean_y) (`KismetMathLibrary.BreakVector2D` (`self.Lean`)))
  (bind (_returnvalue_roll _returnvalue_pitch _returnvalue_yaw) (`KismetMathLibrary.BreakRotator` (`KismetMathLibrary.NormalizedDeltaRotator` _lastvelocityrotation (`self.PreviousVelocityRotation`))))
  (bind (_returnvalue_roll_2 _returnvalue_pitch_2 _returnvalue_yaw_2) (`KismetMathLibrary.BreakRotator` (`Actor.K2_GetActorRotation` (`self.BP_Player`))))
  (bind (_returnvalue_roll_3 _returnvalue_pitch_3) (`KismetMathLibrary.BreakRotator` (`KismetMathLibrary.Conv_VectorToRotator` (`Actor.GetVelocity` (`self.BP_Player`)))))
  (`|ExecutionSequence`
    (:`then_0`
      (if (!= (`KismetMathLibrary.VSize` (`Actor.GetVelocity` (`self.BP_Player`))) 0.0)
        _
        (else
          _))
      (set `self.LastVelocityRotation` (`KismetMathLibrary.MakeRotator` _returnvalue_roll_2 _returnvalue_pitch_3 _returnvalue_yaw_2)))
    (:`then_1`
      (bind _output_get (set `self.YawVelocityDifference` (/ _returnvalue_yaw _returnvalue_2)))
      (bind _output_get_2 (set `self.PitchVelocityDifference` (/ _returnvalue_pitch _returnvalue_2)))
      (set `self.PreviousVelocityRotation` _lastvelocityrotation)
      (set `self.Lean` (`KismetMathLibrary.MakeVector2D` (`KismetMathLibrary.FInterpTo` _lean_x (`KismetMathLibrary.MapRangeClamped` _output_get -180.0 180.0 -1.0 1.0) _returnvalue 5.0) (`KismetMathLibrary.FInterpTo` _lean_y (`KismetMathLibrary.MapRangeClamped` _output_get_2 -180.0 180.0 -1.0 1.0) _returnvalue 15.0))))
    (:`then_2`
      (set `self.LookAtLocation` (select `bool` (`self.bAiming`) :`false` (`KismetMathLibrary.VInterpTo` (`self.LookAtLocation`) (+ (`Actor.K2_GetActorLocation` _bp_player) (* (`Actor.GetActorForwardVector` _bp_player) 5000.0) (0.0 0.0 -2000.0)) (`GameplayStatics.GetWorldDeltaSeconds`) 10.0) :`true` (+ (`SceneComponent.GetSocketLocation` (`Character.Mesh` _bp_player_2) "Head") (* (`SceneComponent.GetForwardVector` (`Actor.RootComponent` _bp_player_2)) 5000.0)))))))

(event `SetActiveComponent`
  (params (UseActiveDelay :type Boolean) (DelayDuration :type "Float (double-precision)") (Component :type "ActorComponent Object Reference") (bNewActive :type Boolean) (bReset :type Boolean))
  (`/Engine/EditorBlueprintResources/StandardMacros.IsValid` Component
    (:`Is Valid`
      (if UseActiveDelay
        (`KismetSystemLibrary.Delay` DelayDuration))
      (`self.SetActive` Component bNewActive bReset))))

(event `SetCameraFOV`
  (params (SavedFOV :type "Float (double-precision)") (FOV_LerpSpeed :type "Float (double-precision)"))
  (if (`self.Use Camera FOV`)
    (set `self.Saved FOV` SavedFOV)
    (set `self.FOV Lerp Speed` FOV_LerpSpeed)
    (`self.SetCameraFOV_Lerp`)))

(event `SetCameraFOV_Lerp`
  (if (not (`KismetMathLibrary.NearlyEqual_FloatFloat` (`CameraComponent.FieldOfView` (`/Game/BP/Character/BP_Player.Camera` (`self.BP_Player`))) (`self.Saved FOV`) 0.1)) :!label _label_3
    (`|ExecutionSequence`
      (:`then_0`
        (set `CameraComponent.FieldOfView` (`KismetMathLibrary.FInterpTo` (`CameraComponent.FieldOfView` (`/Game/BP/Character/BP_Player.Camera` (`self.BP_Player`))) (`self.Saved FOV`) (`GameplayStatics.GetWorldDeltaSeconds`) (`self.FOV Lerp Speed`)) (`/Game/BP/Character/BP_Player.Camera` (`self.BP_Player`))))
      (:`then_1`
        (`KismetSystemLibrary.Delay` 0.0)
        (goto _label_3)))))

(fn `Check Movement Mode`
  (params (MovementMode :type "EMovementMode Enum" :default "MOVE_None"))
  (returns (ReturnValue :type Boolean))
  (return (`|EnumEquality` (`CharacterMovementComponent.MovementMode` (`self.BP_CharacterMovement`)) MovementMode)))

(fn `Get Flight Under Dust `
  (params (PhysicalSurfaceType :type "EPhysicalSurface Enum" :default "SurfaceType_Default"))
  (returns (UnderDust :type "NiagaraComponent Object Reference"))
  (return (`|GetArrayItem` (`self.UnderDustRef`) (select `EPhysicalSurface` PhysicalSurfaceType :`SurfaceType2` 1 :`SurfaceType3` 2 :`SurfaceType4` 3 :`SurfaceType5` 4))))

(fn `Get Lnading VFX`
  (params (PhysicalSurfaceType :type "EPhysicalSurface Enum" :default "SurfaceType_Default"))
  (returns (SuperheroLnading :type "NiagaraSystem Object Reference"))
  (return (`|GetArrayItem` (`self.SuperheroLnading`) (select `EPhysicalSurface` PhysicalSurfaceType :`SurfaceType2` 1 :`SurfaceType3` 2 :`SurfaceType4` 3 :`SurfaceType5` 4))))

(fn `Notifi Line Trace to Up Vector`
  (params (VectorLength :type "Float (double-precision)"))
  (returns (OnHit :type Boolean) (OutHit :type "HitResult Structure"))
  (bind _bp_player (`self.BP_Player`))
  (bind _returnvalue (`Actor.K2_GetActorLocation` _bp_player))
  (`/Engine/EditorBlueprintResources/StandardMacros.IsValid` (`self.BP_Player`)
    (:`Is Valid`
      (bind (_outhit _returnvalue_2) (`KismetSystemLibrary.LineTraceSingle` _returnvalue (+ _returnvalue (* (`Actor.GetActorUpVector` _bp_player) (`local.VectorLength`))) "TraceTypeQuery1" false (`|MakeArray` (`self.BP_Player`) :!type "Actor Object Reference")))
      (return _returnvalue_2 _outhit))))

(fn `Set Aiming`
  (params (IsAiming :type Boolean))
  (bind _charactermovement (`Character.CharacterMovement` (`self.BP_Player`)))
  (bind _springarm (`/Game/BP/Character/BP_Player.SpringArm` (`self.BP_Player`)))
  (bind _springarm_2 (`/Game/BP/Character/BP_Player.SpringArm` (`self.BP_Player`)))
  (bind _output_get (set `self.bAiming` IsAiming))
  (if _output_get
    (bind _output_get_2 (set `CharacterMovementComponent.bUseControllerDesiredRotation` true _charactermovement))
    (set `CharacterMovementComponent.bOrientRotationToMovement` (not _output_get_2) _charactermovement)
    (set `SpringArmComponent.bEnableCameraLag` false _springarm_2)
    (set `SpringArmComponent.bEnableCameraRotationLag` false _springarm_2)
    (set `SpringArmComponent.TargetArmLength` 200.0 _springarm)
    (set `SpringArmComponent.SocketOffset` (0.0 100.0 20.0) _springarm)
    (else
      (bind _output_get_3 (set `CharacterMovementComponent.bUseControllerDesiredRotation` false _charactermovement))
      (set `CharacterMovementComponent.bOrientRotationToMovement` (not _output_get_3) _charactermovement)
      (set `SpringArmComponent.bEnableCameraLag` true _springarm_2)
      (set `SpringArmComponent.bEnableCameraRotationLag` true _springarm_2)
      (set `SpringArmComponent.TargetArmLength` 300.0 _springarm)
      (set `SpringArmComponent.SocketOffset` (0.0 0.0 0.0) _springarm))))

(fn `Set CharacterMovement`
  (params (NewMovementMode :type "EMovementMode Enum" :default "MOVE_None"))
  (bind _bp_charactermovement (`self.BP_CharacterMovement`))
  (`/Engine/EditorBlueprintResources/StandardMacros.IsValid` _bp_charactermovement
    (:`Is Valid`
      (`CharacterMovementComponent.SetMovementMode` _bp_charactermovement NewMovementMode 0))))

(fn `Set Flight Movement Param`
  (params (bFlying :type Boolean))
  (bind ((`Flight_FlightBrakingDeceleration_51_72D08E884DEEF2AAEBE249A83C5FE3DF` _flight_flightbrakingdeceleration) (`Flight_RotationRate_52_031D171243F9AFBB0EE257B4126DF911` _flight_rotationrate)) (break `/Game/BP/Data/FFlight/FFlight` (`self.FFlight`)))
  (bind ((`Flight_FlySpeed_50_D2785AF544622FA8AB4B9A84D7D4764B` _flight_flyspeed) (`Flight_Acceleration_44_FCEAE7124381E9C53E1561B947F7759C` _flight_acceleration)) (break `/Game/BP/Data/FFlight/FFlight` (`self.FFlight`)))
  (bind ((`Flight_FlightBrakingDeceleration_51_72D08E884DEEF2AAEBE249A83C5FE3DF` _flight_flightbrakingdeceleration_2) (`Flight_RotationRate_52_031D171243F9AFBB0EE257B4126DF911` _flight_rotationrate_2)) (break `/Game/BP/Data/FFlight/FFlight` (`self.FFlight`)))
  (bind ((`Flight_FlySpeed_50_D2785AF544622FA8AB4B9A84D7D4764B` _flight_flyspeed_2) (`Flight_Acceleration_44_FCEAE7124381E9C53E1561B947F7759C` _flight_acceleration_2)) (break `/Game/BP/Data/FFlight/FFlight` (`self.FFlight`)))
  (if bFlying
    (set `CharacterMovementComponent.MaxFlySpeed` _flight_flyspeed (`self.BP_CharacterMovement`))
    (set `CharacterMovementComponent.MaxAcceleration` _flight_acceleration (`self.BP_CharacterMovement`))
    (set `CharacterMovementComponent.BrakingDecelerationFlying` _flight_flightbrakingdeceleration_2 (`self.BP_CharacterMovement`))
    (set `CharacterMovementComponent.RotationRate` _flight_rotationrate_2 (`self.BP_CharacterMovement`))
    (else
      (set `CharacterMovementComponent.MaxFlySpeed` _flight_flyspeed_2 (`self.BP_CharacterMovement`))
      (set `CharacterMovementComponent.MaxAcceleration` _flight_acceleration_2 (`self.BP_CharacterMovement`))
      (set `CharacterMovementComponent.BrakingDecelerationFlying` _flight_flightbrakingdeceleration (`self.BP_CharacterMovement`))
      (set `CharacterMovementComponent.RotationRate` _flight_rotationrate (`self.BP_CharacterMovement`)))))

(fn `Set Flying`
  (params (IsFlying :type Boolean))
  (bind _output_get (set `self.bFlying` IsFlying))
  (if _output_get
    (`self.Set CharacterMovement` "MOVE_Flying")
    (else
      (`self.Set CharacterMovement` "MOVE_Falling"))))

(fn `SetSprint`
  (params (IsSprint :type Boolean))
  (locals (MainSprint :type Boolean))
  (bind _bp_charactermovement (`self.BP_CharacterMovement`))
  (bind _issprint (`local.IsSprint`))
  (bind ((`Sprint_FlySpeed_23_7E68750F49C9DC5CC3FFCD8A23C38C86` _sprint_flyspeed) (`Sprint_Acceleration_25_72D08E884DEEF2AAEBE249A83C5FE3DF` _sprint_acceleration)) (break `/Game/BP/Data/FFlight/FFlight_Sprint` (`self.FFlight_Sprint`)))
  (bind _charactermovement (`Character.CharacterMovement` (`self.BP_Player`)))
  (set `local.MainSprint` (`self.bSprint`))
  (if (or (`self.Check Movement Mode` "MOVE_Falling") (`self.Check Movement Mode` "MOVE_Flying"))
    (bind _output_get (set `self.bSprint` (`local.IsSprint`)))
    (bind _output_get_2 (set `CharacterMovementComponent.bOrientRotationToMovement` (not _output_get) _bp_charactermovement))
    (set `CharacterMovementComponent.bUseControllerDesiredRotation` (not _output_get_2) _bp_charactermovement)
    (if (`local.IsSprint`)
      (set `CharacterMovementComponent.MaxWalkSpeed` (`.Sprint_FlyWalkSpeed_49_C8EB5B934AED04DDEC36D0B996605D06` (break `/Game/BP/Data/FFlight/FFlight_Sprint` (`self.FFlight_Sprint`))) (`self.BP_CharacterMovement`))
      (set `CharacterMovementComponent.MaxFlySpeed` _sprint_flyspeed (`self.BP_CharacterMovement`))
      (set `CharacterMovementComponent.MaxAcceleration` _sprint_acceleration (`self.BP_CharacterMovement`))
      (set `CharacterMovementComponent.RotationRate` (`.Sprint_RotationRate_27_031D171243F9AFBB0EE257B4126DF911` (break `/Game/BP/Data/FFlight/FFlight_Sprint` (`self.FFlight_Sprint`))) (`self.BP_CharacterMovement`))
      (bind _output_get_3 (set `CharacterMovementComponent.bUseControllerDesiredRotation` _issprint _charactermovement))
      (set `CharacterMovementComponent.bOrientRotationToMovement` (not _output_get_3) _charactermovement)
      (`self.SetActiveComponent` false 0.0 (`self.FlightWaveRef`) true true)
      (`/Game/BP/Character/Object/Wings/BP_Wings.Wings Start Sprint` (`/Game/BP/Character/BP_Player.Wings` (`self.BP_Player`)))
      (`self.Stop To Play Anim` "/Game/Animation/Player/Flight/C_Flight_FastMove_Start_C_Montage.C_Flight_FastMove_Start_C_Montage")
      (else
        (set `CharacterMovementComponent.MaxWalkSpeed` (`.Unarmed_FlyWarkSpeed_31_15D920654182E164BAA33FBCB472357A` (break `/Game/BP/Data/FFlight/FUnarmed` (`self.FUnarmed`))) (`self.BP_CharacterMovement`))
        (set `CharacterMovementComponent.MaxFlySpeed` (`.Flight_FlySpeed_50_D2785AF544622FA8AB4B9A84D7D4764B` (break `/Game/BP/Data/FFlight/FFlight` (`self.FFlight`))) (`self.BP_CharacterMovement`))
        (set `CharacterMovementComponent.MaxAcceleration` (`.Flight_Acceleration_44_FCEAE7124381E9C53E1561B947F7759C` (break `/Game/BP/Data/FFlight/FFlight` (`self.FFlight`))) (`self.BP_CharacterMovement`))
        (set `CharacterMovementComponent.RotationRate` (`.Flight_RotationRate_52_031D171243F9AFBB0EE257B4126DF911` (break `/Game/BP/Data/FFlight/FFlight` (`self.FFlight`))) (`self.BP_CharacterMovement`))
        (bind _output_get_4 (set `CharacterMovementComponent.bUseControllerDesiredRotation` _issprint _charactermovement))
        (set `CharacterMovementComponent.bOrientRotationToMovement` (not _output_get_4) _charactermovement)
        (`self.SetActiveComponent` false 0.0 (`self.FlightWaveRef`))
        (`/Game/BP/Character/Object/Wings/BP_Wings.Set Sprint` (`/Game/BP/Character/BP_Player.Wings` (`self.BP_Player`)) false)
        (if (`local.MainSprint`)
          (if (`self.bLanding`)
            (`self.Stop To Play Anim` "/Game/Animation/Player/Flight/C_Landing_C_Montage.C_Landing_C_Montage")
            (set `self.bLanding` false)
            (else
              (`self.Stop To Play Anim` "/Game/Animation/Player/Flight/C_Flight_Hover_Start_C_Montage.C_Flight_Hover_Start_C_Montage"))))))))

(fn `Spawn Niagara At Location Or Attach`
  (params (IsAttach :type Boolean) (AttachToComponent :type "SceneComponent Object Reference") (SystemTemplate :type "NiagaraSystem Object Reference") (Location :type "Vector Structure") (Rotation :type "Rotator Structure"))
  (returns (ReturnValue :type "NiagaraComponent Object Reference"))
  (if IsAttach
    (bind _returnvalue (`NiagaraFunctionLibrary.SpawnSystemAttached` SystemTemplate AttachToComponent "None" Location Rotation "KeepRelativeOffset" true))
    (return _returnvalue)
    (else
      (bind _returnvalue_2 (`NiagaraFunctionLibrary.SpawnSystemAtLocation` SystemTemplate Location Rotation))
      (return _returnvalue_2))))

(fn `Stop To Play Anim`
  (params (`In Anim` :type "AnimMontage Object Reference"))
  (bind _bp_player (`self.BP_Player`))
  (`Character.StopAnimMontage` _bp_player null)
  (`Character.PlayAnimMontage` _bp_player `In Anim` 1.0 "None"))