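; BP_PatroComponent is an AI component that tracks an actor's current point along a spline-based PatrolPath.
; It exposes path validity, point count and the current point's world location, returning zero values when no path is set.
; UpdateNextIndex steps the index in the current direction, wrapping on closed-loop splines and ping-ponging on open ones via a Reverse flag.
; It performs no movement itself, and BeginPlay and Tick are empty.
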(fn `Get Spline Index Location`
  (returns (ReturnValue :type "Vector Structure"))
  (if (`self.IsPathValid`)
    (return (`SplineComponent.GetLocationAtSplinePoint` (`/Game/BP/Character/Object/PatrolPath/BP_PatrolPath.Spline` (`self.PatrolPath`)) (`self.Index`) "World"))
    (else
      (return (0.0 0.0 0.0)))))

(fn `Get Spline Point Count`
  (returns (ReturnValue :type Integer))
  (if (`self.IsPathValid`)
    (return (`SplineComponent.GetNumberOfSplinePoints` (`/Game/BP/Character/Object/PatrolPath/BP_PatrolPath.Spline` (`self.PatrolPath`))))
    (else
      (return 0))))

(fn `IsPathValid`
  (returns (ReturnValue :type Boolean))
  (return (`KismetSystemLibrary.IsValid` (`self.PatrolPath`))))

(fn `Update Next Index`
  (if (`self.IsPathValid`)
    (if (`self.bReverse`)
      ;[1 1 1] 역방향
      (if (<= (`self.Index`) 0)
        (if (`SplineComponent.IsClosedLoop` (`/Game/BP/Character/Object/PatrolPath/BP_PatrolPath.Spline` (`self.PatrolPath`)))
          (set `self.Index` (- (`self.Get Spline Point Count`) 1))
          (else
            (set `self.Index` 1)
            (set `self.bReverse` false)))
        (else
          (`/Engine/EditorBlueprintResources/StandardMacros.DecrementInt` (`self.Index`))))
      (else
        ;[1 1 1] 정방향
        (if (>= (`self.Index`) (- (`self.Get Spline Point Count`) 1))
          (if (`SplineComponent.IsClosedLoop` (`/Game/BP/Character/Object/PatrolPath/BP_PatrolPath.Spline` (`self.PatrolPath`)))
            (set `self.Index` 0)
            (else
              (set `self.Index` (- (`self.Get Spline Point Count`) 2))
              (set `self.bReverse` true)))
          (else
            (`/Engine/EditorBlueprintResources/StandardMacros.IncrementInt` (`self.Index`))))))))