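; BP_WidgetComponent is a player component that creates and controls the HUD and weapon choice screen for BP_Player.
; On BeginPlay it adds the main widget, seeding its HP bar from the status component, plus a hidden weapon choice widget.
; Opening weapon choice slows time and shows a centered, locked cursor; closing restores play and passes the selection to the melee component.
; It also toggles the interaction prompt with key and object name.
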(event `self.ReceiveBeginPlay`
  (bind _bp_statuscomponent (`/Game/BP/Character/BP_Character.BP_StatusComponent` (`self.BP_Player`)))
  (bind _asbp_player (cast `/Game/BP/Character/BP_Player` (`self.GetOwner`)))
  (set `self.BP_Player` _asbp_player)
  (`|ExecutionSequence`
    (:`then_0`
      (bind `_as플레이어_컨트롤러` (cast `PlayerController` (`Pawn.GetController` (`self.BP_Player`))))
      (set `self.PalyerController` `_as플레이어_컨트롤러`)
      (`|ExecutionSequence`
        (:`then_0`
          (bind _returnvalue (`|CreateWidget` "/Game/BP/Widget/WB_MainWidget.WB_MainWidget_C" (`self.PalyerController`)))
          (bind _output_get (set `self.Main Widget` _returnvalue))
          (`UserWidget.AddToViewport` _output_get 0)
          (`Widget.SetVisibility` (`self.Main Widget`) "Visible")
          (`/Game/BP/Widget/WB_MainWidget.Widget Set Owner` (`self.Main Widget`) (`self.BP_Player`))
          (`/Game/BP/Widget/WB_HPBar.Begin HPBar` (`/Game/BP/Widget/WB_MainWidget.WB_HPBer` (`self.Main Widget`)) (`/Game/BP/Components/BP_StatusComponent.Stat HP Max` _bp_statuscomponent) (`/Game/BP/Components/BP_StatusComponent.Stat HP` _bp_statuscomponent)))
        (:`then_1`
          (bind _returnvalue_2 (`|CreateWidget` "/Game/BP/Widget/WB_Weapon_Choice.WB_Weapon_Choice_C" (`self.PalyerController`)))
          (bind _output_get_2 (set `self.Weapon Choice Widget` _returnvalue_2))
          (`UserWidget.AddToViewport` _output_get_2 0)
          (`Widget.SetVisibility` (`self.Weapon Choice Widget`) "Hidden"))))))

(fn `Get Screen Center`
  (returns (`Screen Center X` :type "Float (double-precision)") (`Screen Center Y` :type "Float (double-precision)"))
  (bind (_returnvalue_x _returnvalue_y) (`KismetMathLibrary.BreakVector2D` (/ (`WidgetLayoutLibrary.GetViewportSize`) (2.0 2.0))))
  (return _returnvalue_x _returnvalue_y))

(fn `See Weapon Choice Widget`
  (params (`In Value` :type Boolean))
  (bind (_screen_center_x _screen_center_y) (`self.Get Screen Center`))
  (bind _in_value (`local.In Value`))
  (bind _weapon_choice_widget (`self.Weapon Choice Widget`))
  (if `In Value`
    (`PlayerController.SetMouseLocation` (`GameplayStatics.GetPlayerController` 0) (`KismetMathLibrary.FTrunc` _screen_center_x) (`KismetMathLibrary.FTrunc` _screen_center_y))
    (`GameplayStatics.SetGlobalTimeDilation` 0.1)
    (`Widget.SetVisibility` _weapon_choice_widget "Visible")
    (`self.Set MouseCurset` _in_value)
    (else
      (`GameplayStatics.SetGlobalTimeDilation` 1.0)
      (`Widget.SetVisibility` _weapon_choice_widget "Hidden")
      (`self.Set MouseCurset` _in_value)
      (`/Game/BP/Components/BP_MeleeCompoent.Change Weapon` (`/Game/BP/Character/BP_Character.BP_MeleeCompoent` (`self.BP_Player`)) (`/Game/BP/Widget/WB_Weapon_Choice.GetEStateType` (`self.Weapon Choice Widget`))))))

(fn `Set Interaction`
  (params (`In Interaction` :type "/Game/BP/Interaction/BP_Interaction Object Reference") (`On Interaction` :type Boolean))
  (if `On Interaction`
    (set `TextBlock.Text` "F" (`/Game/BP/Widget/WB_Interaction_Widget.InputKeyText` (`/Game/BP/Widget/WB_MainWidget.WB_Interaction_Widget` (`self.Main Widget`))))
    (set `TextBlock.Text` (`/Game/BP/Interaction/BP_Interaction.Object Name Text` (`local.In Interaction`)) (`/Game/BP/Widget/WB_Interaction_Widget.ObjectNameText` (`/Game/BP/Widget/WB_MainWidget.WB_Interaction_Widget` (`self.Main Widget`))))
    (`Widget.SetVisibility` (`/Game/BP/Widget/WB_MainWidget.WB_Interaction_Widget` (`self.Main Widget`)) "Visible")
    (else
      (`Widget.SetVisibility` (`/Game/BP/Widget/WB_MainWidget.WB_Interaction_Widget` (`self.Main Widget`)) "Hidden"))))

(fn `Set MouseCurset`
  (params (`In Value` :type Boolean))
  (bind _returnvalue (`GameplayStatics.GetPlayerController` 0))
  (bind _returnvalue_2 (`GameplayStatics.GetPlayerController` 0))
  (if `In Value`
    (set `PlayerController.bShowMouseCursor` true _returnvalue_2)
    (`WidgetBlueprintLibrary.SetInputMode_GameAndUIEx` _returnvalue_2 null "LockAlways")
    (else
      (set `PlayerController.bShowMouseCursor` false _returnvalue)
      (`WidgetBlueprintLibrary.SetInputMode_GameOnly` _returnvalue))))