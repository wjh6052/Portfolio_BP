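; Damage component on BP_Melee that computes attack damage, knockback and critical hits for its owning BP_Character.
; GetAttackDamage picks run-to-attack, jump, combo or skill data from the weapon's data asset, then adds the character's damage stat.
; Melee hits roll criticals from attack and status crit values, though jump hits never report them; projectiles skip the roll and add 70% of the stat.
; GetKnockBack builds a forward-plus-up vector from an actor's orientation.
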(event `self.ReceiveBeginPlay`
  (bind _asbp_melee (cast `/Game/BP/Melee/BP_Melee` (`self.GetOwner`)))
  (bind _output_get (set `self.BP_Melee` _asbp_melee))
  (set `self.Data Asset` (`/Game/BP/Melee/BP_Melee.DA_Data Asset` _output_get))
  (bind _asbp_character (cast `/Game/BP/Character/BP_Character` (`Actor.GetOwner` (`self.BP_Melee`))))
  (set `self.BP Character` _asbp_character))

(fn `Check Critical Damage Knock Back `
  (params (`In Skill Data` :type "/Game/BP/Data/DataAsset/Melee/DTS_SkillDatas Structure") (`In Action Data` :type "/Game/BP/Data/DataAsset/Melee/DTS_ActionDatas Structure") (`In Skill` :type Boolean) (`In Jump` :type Boolean) (`In Run To Attack` :type Boolean) (`In Jump Action` :type Boolean))
  (returns (Damage :type "Float (double-precision)") (`Knock Back Forward` :type "Float (double-precision)") (`Knock Back UP` :type "Float (double-precision)") (`On Critical` :type Boolean))
  (locals (`Damage Value` :type "Float (double-precision)"))
  (bind (_in_action_data_animmontage _in_action_data_playrate _in_action_data_damage _in_action_data_projectiledamage _in_action_data_critical _in_action_data_knockback_forward _in_action_data_knock_back_up) (break `/Game/BP/Data/DataAsset/Melee/DTS_ActionDatas` (`local.In Action Data`)))
  (bind (_in_action_data_animmontage_2 _in_action_data_playrate_2 _in_action_data_damage_2 _in_action_data_projectiledamage_2 _in_action_data_critical_2 _in_action_data_knockback_forward_2 _in_action_data_knock_back_up_2) (break `/Game/BP/Data/DataAsset/Melee/DTS_ActionDatas` (`local.In Action Data`)))
  (bind (_in_skill_data_skillnumber _in_skill_data_animmontage _in_skill_data_damage _in_skill_data_projectiledamage _in_skill_data_critical _in_skill_data_playrate _in_skill_data_knockback_forward _in_skill_data_knock_back_up) (break `/Game/BP/Data/DataAsset/Melee/DTS_SkillDatas` (`local.In Skill Data`)))
  (bind (_in_action_data_animmontage_3 _in_action_data_playrate_3 _in_action_data_damage_3 _in_action_data_projectiledamage_3 _in_action_data_critical_3 _in_action_data_knockback_forward_3 _in_action_data_knock_back_up_3) (break `/Game/BP/Data/DataAsset/Melee/DTS_ActionDatas` (`local.In Action Data`)))
  (bind (_in_action_data_animmontage_4 _in_action_data_playrate_4 _in_action_data_damage_4 _in_action_data_projectiledamage_4 _in_action_data_critical_4) (break `/Game/BP/Data/DataAsset/Melee/DTS_ActionDatas` (`local.In Action Data`)))
  (bind (_in_action_data_animmontage_5 _in_action_data_playrate_5 _in_action_data_damage_5 _in_action_data_projectiledamage_5 _in_action_data_critical_5) (break `/Game/BP/Data/DataAsset/Melee/DTS_ActionDatas` (`local.In Action Data`)))
  (bind (_in_skill_data_skillnumber_2 _in_skill_data_animmontage_2 _in_skill_data_damage_2 _in_skill_data_projectiledamage_2 _in_skill_data_critical_2) (break `/Game/BP/Data/DataAsset/Melee/DTS_SkillDatas` (`local.In Skill Data`)))
  (bind (_in_action_data_animmontage_6 _in_action_data_playrate_6 _in_action_data_damage_6 _in_action_data_projectiledamage_6 _in_action_data_critical_6) (break `/Game/BP/Data/DataAsset/Melee/DTS_ActionDatas` (`local.In Action Data`)))
  (if `In Jump`
    (set `local.Damage Value` _in_action_data_damage_4)
    (if (>= (+ _in_action_data_critical_4 (`/Game/BP/Components/BP_StatusComponent.Stat Critical Chance` (`/Game/BP/Character/BP_Character.BP_StatusComponent` (`self.BP Character`)))) (`KismetMathLibrary.RandomFloatInRange` 0.0 100.0))
      (return (* (`local.Damage Value`) (/ (+ (`/Game/BP/Components/BP_StatusComponent.Stat Critical Damage` (`/Game/BP/Character/BP_Character.BP_StatusComponent` (`self.BP Character`))) 150.0) 100.0)) _in_action_data_knockback_forward _in_action_data_knock_back_up true)
      (else
        (return (`local.Damage Value`) _in_action_data_knockback_forward _in_action_data_knock_back_up false)))
    (elif `In Run To Attack`
      (set `local.Damage Value` _in_action_data_damage_5)
      (if (>= (+ _in_action_data_critical_5 (`/Game/BP/Components/BP_StatusComponent.Stat Critical Chance` (`/Game/BP/Character/BP_Character.BP_StatusComponent` (`self.BP Character`)))) (`KismetMathLibrary.RandomFloatInRange` 0.0 100.0))
        (return (* (`local.Damage Value`) (/ (+ (`/Game/BP/Components/BP_StatusComponent.Stat Critical Damage` (`/Game/BP/Character/BP_Character.BP_StatusComponent` (`self.BP Character`))) 150.0) 100.0)) _in_action_data_knockback_forward_2 _in_action_data_knock_back_up_2 true)
        (else
          (return (`local.Damage Value`) _in_action_data_knockback_forward_2 _in_action_data_knock_back_up_2 false)))
      (elif (`local.In Skill`)
        (set `local.Damage Value` _in_skill_data_damage_2)
        (if (>= (+ _in_skill_data_critical_2 (`/Game/BP/Components/BP_StatusComponent.Stat Critical Chance` (`/Game/BP/Character/BP_Character.BP_StatusComponent` (`self.BP Character`)))) (`KismetMathLibrary.RandomFloatInRange` 0.0 100.0))
          (return (* (`local.Damage Value`) (/ (+ (`/Game/BP/Components/BP_StatusComponent.Stat Critical Damage` (`/Game/BP/Character/BP_Character.BP_StatusComponent` (`self.BP Character`))) 150.0) 100.0)) _in_skill_data_knockback_forward _in_skill_data_knock_back_up true)
          (else
            (return (`local.Damage Value`) _in_skill_data_knockback_forward _in_skill_data_knock_back_up false)))
        (else
          (set `local.Damage Value` _in_action_data_damage_6)
          (if (>= (+ _in_action_data_critical_6 (`/Game/BP/Components/BP_StatusComponent.Stat Critical Chance` (`/Game/BP/Character/BP_Character.BP_StatusComponent` (`self.BP Character`)))) (`KismetMathLibrary.RandomFloatInRange` 0.0 100.0))
            (return (* (`local.Damage Value`) (/ (+ (`/Game/BP/Components/BP_StatusComponent.Stat Critical Damage` (`/Game/BP/Character/BP_Character.BP_StatusComponent` (`self.BP Character`))) 150.0) 100.0)) _in_action_data_knockback_forward_3 _in_action_data_knock_back_up_3 true)
            (else
              (return (`local.Damage Value`) _in_action_data_knockback_forward_3 _in_action_data_knock_back_up_3 false))))))))

(fn `Get Attack Damage`
  (params (`In Combo Count` :type Integer) (`In Skill Count` :type Integer) (`In Skill Number` :type Integer) (`In Jump Action` :type Boolean) (`In Projectile` :type Boolean) (`In Skill` :type Boolean) (`In Run To Attack` :type Boolean))
  (returns (Damage :type "Float (double-precision)") (` Knock Back Forward` :type "Float (double-precision)") (`Knock Back UP` :type "Float (double-precision)") (`On Critical` :type Boolean))
  (bind (_jump_action_animmontage _jump_action_playrate _jump_action_damage _jump_action_projectiledamage _jump_action_critical _jump_action_knockback_forward _jump_action_knock_back_up) (break `/Game/BP/Data/DataAsset/Melee/DTS_ActionDatas` (`/Game/BP/Data/DataAsset/Melee/DABP_Melee.Jump Action` (`/Game/BP/Melee/BP_Melee.DA_Data Asset` (`self.BP_Melee`)))))
  (bind (_output_animmontage _output_playrate _output_damage _output_projectiledamage _output_critical _output_knockback_forward _output_knock_back_up) (break `/Game/BP/Data/DataAsset/Melee/DTS_ActionDatas` (`|GetArrayItem` (`/Game/BP/Data/DataAsset/Melee/DABP_Melee.Action` (`/Game/BP/Melee/BP_Melee.DA_Data Asset` (`self.BP_Melee`))) (`local.In Combo Count`))))
  (if (`local.In Run To Attack`)
    (bind (_damage _knock_back_forward _knock_back_up _on_critical) (`self.Check Critical Damage Knock Back ` (struct) (`/Game/BP/Data/DataAsset/Melee/DABP_Melee.Run To Attack` (`/Game/BP/Melee/BP_Melee.DA_Data Asset` (`self.BP_Melee`))) false false true))
    (return (+ _damage (`/Game/BP/Components/BP_StatusComponent.Stat Damage` (`/Game/BP/Character/BP_Character.BP_StatusComponent` (`self.BP Character`)))) _knock_back_forward _knock_back_up _on_critical)
    (elif (`local.In Projectile`)
      (if (`local.In Jump Action`)
        (return (+ _jump_action_projectiledamage (* (`/Game/BP/Components/BP_StatusComponent.Stat Damage` (`/Game/BP/Character/BP_Character.BP_StatusComponent` (`self.BP Character`))) 0.7)) _jump_action_knockback_forward _jump_action_knock_back_up false)
        (elif (`local.In Skill`)
          (bind _skill (`self.Get Skill` (`local.In Skill Number`) (`local.In Skill Count`) (`local.In Projectile`)))
          (return (+ (`.ProjectileDamage_31_D52D50C240A1393D98366A892BF77316` (break `/Game/BP/Data/DataAsset/Melee/DTS_SkillDatas` _skill)) (* (`/Game/BP/Components/BP_StatusComponent.Stat Damage` (`/Game/BP/Character/BP_Character.BP_StatusComponent` (`self.BP Character`))) 0.7)) (`.KnockBack_Forward_23_3D7BC9B14C293CE46F68EE8E87C8A15C` (break `/Game/BP/Data/DataAsset/Melee/DTS_SkillDatas` _skill)) (`.Knock_Back_UP_22_1F5431B843214E0A494DC38044CDA4E2` (break `/Game/BP/Data/DataAsset/Melee/DTS_SkillDatas` _skill)) false)
          (else
            (return (+ _output_projectiledamage (* (`/Game/BP/Components/BP_StatusComponent.Stat Damage` (`/Game/BP/Character/BP_Character.BP_StatusComponent` (`self.BP Character`))) 0.7)) _output_knockback_forward _output_knock_back_up false))))
      (elif (`local.In Jump Action`)
        (bind (_damage_2 _knock_back_forward_2 _knock_back_up_2) (`self.Check Critical Damage Knock Back ` (struct) (`/Game/BP/Data/DataAsset/Melee/DABP_Melee.Jump Action` (`/Game/BP/Melee/BP_Melee.DA_Data Asset` (`self.BP_Melee`))) false true))
        (return (+ _damage_2 (`/Game/BP/Components/BP_StatusComponent.Stat Damage` (`/Game/BP/Character/BP_Character.BP_StatusComponent` (`self.BP Character`)))) _knock_back_forward_2 _knock_back_up_2 false)
        (elif (`local.In Skill`)
          (bind _skill_2 (`self.Get Skill` (`local.In Skill Number`) (`local.In Skill Count`) (`local.In Projectile`)))
          (bind (_damage_3 _knock_back_forward_3 _knock_back_up_3 _on_critical_2) (`self.Check Critical Damage Knock Back ` _skill_2 (struct) true))
          (return (+ _damage_3 (`/Game/BP/Components/BP_StatusComponent.Stat Damage` (`/Game/BP/Character/BP_Character.BP_StatusComponent` (`self.BP Character`)))) _knock_back_forward_3 _knock_back_up_3 _on_critical_2)
          (else
            (bind (_damage_4 _knock_back_forward_4 _knock_back_up_4 _on_critical_3) (`self.Check Critical Damage Knock Back ` (struct) (`|GetArrayItem` (`/Game/BP/Data/DataAsset/Melee/DABP_Melee.Action` (`/Game/BP/Melee/BP_Melee.DA_Data Asset` (`self.BP_Melee`))) (`local.In Combo Count`))))
            (return (+ _damage_4 (`/Game/BP/Components/BP_StatusComponent.Stat Damage` (`/Game/BP/Character/BP_Character.BP_StatusComponent` (`self.BP Character`)))) _knock_back_forward_4 _knock_back_up_4 _on_critical_3)))))))

(fn `Get Knock Back`
  (params (`In Owner` :type "/Game/BP/Character/BP_Character Object Reference") (`In Knock Back Forward` :type "Float (double-precision)") (`In Knock Back Up` :type "Float (double-precision)"))
  (returns (Direction :type "Vector Structure"))
  (return (+ (* (`SceneComponent.GetForwardVector` (`Actor.RootComponent` (`local.In Owner`))) (`local.In Knock Back Forward`)) (* (`local.In Knock Back Up`) (`SceneComponent.GetUpVector` (`Actor.RootComponent` (`local.In Owner`)))))))

(fn `Get Skill`
  (params (`In Skill Number` :type Integer) (`In Skill Count` :type Integer) (`In Projectile` :type Boolean))
  (returns (Skill :type "/Game/BP/Data/DataAsset/Melee/DTS_SkillDatas Structure"))
  (if `In Projectile`
    (switch `int` (`local.In Skill Number`)
      (:`0`
        (return (`|GetArrayItem` (`/Game/BP/Data/DataAsset/Melee/DABP_Melee.Skill_1` (`/Game/BP/Melee/BP_Melee.DA_Data Asset` (`self.BP_Melee`))) (`local.In Skill Count`))))
      (:`1`
        (return (`|GetArrayItem` (`/Game/BP/Data/DataAsset/Melee/DABP_Melee.Skill_2` (`/Game/BP/Melee/BP_Melee.DA_Data Asset` (`self.BP_Melee`))) (`local.In Skill Count`))))
      (:`2`
        (return (`|GetArrayItem` (`/Game/BP/Data/DataAsset/Melee/DABP_Melee.Skill_3` (`/Game/BP/Melee/BP_Melee.DA_Data Asset` (`self.BP_Melee`))) (`local.In Skill Count`)))))
    (else
      (switch `int` (`local.In Skill Number`)
        (:`0`
          (return (`|GetArrayItem` (`/Game/BP/Data/DataAsset/Melee/DABP_Melee.Skill_1` (`/Game/BP/Melee/BP_Melee.DA_Data Asset` (`self.BP_Melee`))) (`local.In Skill Count`))))
        (:`1`
          (return (`|GetArrayItem` (`/Game/BP/Data/DataAsset/Melee/DABP_Melee.Skill_2` (`/Game/BP/Melee/BP_Melee.DA_Data Asset` (`self.BP_Melee`))) (`local.In Skill Count`))))
        (:`2`
          (return (`|GetArrayItem` (`/Game/BP/Data/DataAsset/Melee/DABP_Melee.Skill_3` (`/Game/BP/Melee/BP_Melee.DA_Data Asset` (`self.BP_Melee`))) (`local.In Skill Count`))))))))