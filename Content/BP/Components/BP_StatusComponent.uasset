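; BP_StatusComponent is a component that holds the runtime combat stats of its owning BP_Character.
; On BeginPlay it copies HP, max HP, damage, defense and critical values from the character's FStat struct.
; AddDamage subtracts HP, treats negative input as healing capped at max, and on damage exceeding remaining HP zeroes it and calls Dash.
; Dash changes StatusType and forwards to the character's Dash.
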(event `self.ReceiveBeginPlay`
  (bind _asbp_character (cast `/Game/BP/Character/BP_Character` (`self.GetOwner`)))
  (bind _output_get (set `self.BP Character` _asbp_character))
  (bind (_fstat_hp _fstat_hpmax _fstat_damage _fstat_defense _fstat_criticaldamage _fstat_criticalchance) (break `/Game/BP/Data/FFlight/FStat` (`/Game/BP/Character/BP_Character.FStat` _output_get)))
  (set `self.Stat HP` _fstat_hp)
  (set `self.Stat HP Max` _fstat_hpmax)
  (set `self.Stat Damage` _fstat_damage)
  (set `self.Stat Defense` _fstat_defense)
  (set `self.Stat Critical Damage` _fstat_criticaldamage)
  (set `self.Stat Critical Chance` _fstat_criticalchance))

(fn `Add Damage`
  (params (`In Damage` :type "Float (double-precision)"))
  (bind _returnvalue (- (`self.Stat HP`) (`local.In Damage`)))
  (bind _returnvalue_2 (+ (* (`local.In Damage`) -1.0) (`self.Stat HP`)))
  (if (>= (`local.In Damage`) 0.0)
    (if (>= _returnvalue 0.0)
      (set `self.Stat HP` _returnvalue)
      (else
        (set `self.Stat HP` 0.0)
        (`self.Dash `)))
    (elif (<= _returnvalue_2 (`self.Stat HP Max`))
      (set `self.Stat HP` _returnvalue_2)
      (else
        (set `self.Stat HP` (`self.Stat HP Max`))))))

(fn `Dash `
  (set `self.Status Type` "NewEnumerator1")
  (`/Game/BP/Character/BP_Character.Dash ` (`self.BP Character`)))