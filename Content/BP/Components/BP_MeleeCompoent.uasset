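; Character component that owns the melee weapon actors for players and enemies and routes combat actions to the equipped one.
; On BeginPlay it spawns Unarmed and Assassin actors for players, or a Great Sword for enemies.
; ChangeWeapon stops flight, swaps the equipped actor by state and updates the player's skill icon.
; Attacks, cooldown-gated skills, aim, double jump and hit montages delegate to the active weapon.
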(event `self.ReceiveBeginPlay`
  (bind _asbp_character (cast `/Game/BP/Character/BP_Character` (`self.GetOwner`)))
  (set `self.BP_Character` _asbp_character)
  (`|ExecutionSequence`
    (:`then_0`
      (bind _asbp_player (cast `/Game/BP/Character/BP_Player` (`self.BP_Character`)))
      (set `self.BP_Player` _asbp_player)
      (`|ExecutionSequence`
        (:`then_0`
          (bind _returnvalue (`|SpawnActorFromClass` "/Game/BP/Melee/Player/BP_PlayerUnarmed.BP_PlayerUnarmed_C" (`KismetMathLibrary.MakeTransform` (0.0 0.0 0.0)) "Undefined" "MultiplyWithRoot" (`self.GetOwner`) null))
          (bind _output_get (set `self.Unarmed` _returnvalue))
          (`Actor.SetActorHiddenInGame` _output_get true)
          (set `self.Have Melee` (`self.Unarmed`)))
        (:`then_1`
          (bind _returnvalue_2 (`|SpawnActorFromClass` "/Game/BP/Melee/Player/BP_Assassin.BP_Assassin_C" (`KismetMathLibrary.MakeTransform` (0.0 0.0 0.0)) "Undefined" "MultiplyWithRoot" (`self.GetOwner`) null))
          (bind _output_get_2 (set `self.BP_Assassin` _returnvalue_2))
          (`Actor.SetActorHiddenInGame` _output_get_2 true))))
    (:`then_1`
      (bind _asbp_enemy (cast `/Game/BP/Character/Enemy/BP_Enemy` (`self.BP_Character`)))
      (set `self.BP Enemy` _asbp_enemy)
      (`|ExecutionSequence`
        (:`then_0`
          (bind _returnvalue_3 (`|SpawnActorFromClass` "/Game/BP/Melee/Enemy/BP_GreatSword_Melee.BP_GreatSword_Melee_C" (`KismetMathLibrary.MakeTransform` (0.0 0.0 0.0)) "Undefined" "MultiplyWithRoot" (`self.GetOwner`) null))
          (set `self.BP_Great Sword_Melee` _returnvalue_3))))))

(fn `Change Weapon`
  (params (`In State` :type "/Game/BP/Data/Enum/EStateType Enum" :default "NewEnumerator0"))
  (locals (`Before State` :type "/Game/BP/Data/Enum/EStateType Enum" :default "NewEnumerator0") (StateNum :type Integer))
  (bind _out_state (`/Game/BP/Character/BP_Character.Get Player State` (`self.BP_Character`)))
  (if (not (`|EnumEquality` (`local.In State`) _out_state))
    (if (`|EnumEquality` _out_state "NewEnumerator10")
      (`/Game/BP/Components/BP_FlightComponent.StopFlight` (`/Game/BP/Character/BP_Player.BP_FlightComponent` (`self.BP_Player`))))
    (`/Game/BP/Character/BP_Character.Set State` (`self.BP_Character`) (`local.In State`))
    (`/Engine/EditorBlueprintResources/StandardMacros.IsValid` (`self.Have Melee`)
      (:`Is Valid`
        (`/Game/BP/Melee/BP_Melee.Set Equip` (`self.Have Melee`) false))
      (:`Is Not Valid`
        _))
    (switch `/Game/BP/Data/Enum/EStateType` (`local.In State`)
      (:`NewEnumerator0`
        (set `self.Have Melee` (`self.Unarmed`))
        (set `local.StateNum` 0))
      (:`NewEnumerator1`
        (set `self.Have Melee` (`self.BP_Assassin`))
        (set `local.StateNum` 2)
        (`/Game/BP/Melee/BP_Melee.Set Equip` (`self.Have Melee`) true :!label _label))
      (:`NewEnumerator12`
        (set `self.Have Melee` (`self.BP_Great Sword_Melee`))
        (set `local.StateNum` 7)
        (goto _label)))
    (`/Engine/EditorBlueprintResources/StandardMacros.IsValid` (`self.BP_Player`)
      (:`Is Valid`
        (`/Game/BP/Widget/WB_SkillIcon.Set Swizer` (`/Game/BP/Widget/WB_MainWidget.WB_SkillIcon` (`/Game/BP/Components/BP_WidgetComponent.WB_Main Widget` (`/Game/BP/Character/BP_Player.BP_WidgetComponent` (`self.BP_Player`)))) (`local.StateNum`))))))

(fn `Double Jump`
  (set `/Game/BP/Character/BP_Player.bDouble Jump` true (`self.BP_Player`))
  (`/Game/BP/Melee/BP_Melee.Double Jump` (`self.Have Melee`)))

(fn `Hit Montage`
  (bind _have_melee (`self.Have Melee`))
  (bind _bp_character (`self.BP_Character`))
  (`/Engine/EditorBlueprintResources/StandardMacros.IsValid` _have_melee
    (:`Is Valid`
      (`/Game/BP/Character/BP_Character.Set Status` _bp_character "NewEnumerator5")
      (`/Game/BP/Melee/BP_Melee.Hit Montage` _have_melee))
    (:`Is Not Valid`
      (`KismetSystemLibrary.PrintString` "No Have Melee!!")
      (`/Game/BP/Character/BP_Character.Set Status` _bp_character "NewEnumerator0"))))

(fn `Set Aim`
  (params (`In Aim` :type Boolean))
  (`/Engine/EditorBlueprintResources/StandardMacros.IsValid` (`self.Have Melee`)
    (:`Is Valid`
      (`/Game/BP/Melee/BP_Melee.Set Aim` (`self.Have Melee`) (`local.In Aim`)))))

(fn `Start Attack`
  (bind _have_melee (`self.Have Melee`))
  (`/Engine/EditorBlueprintResources/StandardMacros.IsValid` _have_melee
    (:`Is Valid`
      (if (`/Game/BP/Character/BP_Character.Is Status` (`self.BP_Character`) "NewEnumerator15")
        (`/Game/BP/Character/BP_Character.Set Status` (`self.BP_Character`) "NewEnumerator15")
        (else
          (`/Game/BP/Melee/BP_Melee.Attack Action` _have_melee))))))

(fn `Start Skill`
  (params (`Skill Num` :type Integer))
  (`/Engine/EditorBlueprintResources/StandardMacros.IsValid` (`self.Have Melee`)
    (:`Is Valid`
      (if (>= (- (`local.Skill Num`) 1) 0)
        (if (not (`/Game/BP/Melee/BP_Melee.bOnSkill` (`self.Have Melee`)))
          (switch `int` (- (`local.Skill Num`) 1)
            (:`0`
              (if (not (`/Game/BP/Melee/BP_Melee.bOnSkill_1 CooldownTime` (`self.Have Melee`)))
                (`/Game/BP/Melee/BP_Melee.Skill Action` (`self.Have Melee`) (- (`local.Skill Num`) 1))))
            (:`1`
              (if (not (`/Game/BP/Melee/BP_Melee.bOnSkill_2 CooldownTime` (`self.Have Melee`)))
                (`/Game/BP/Melee/BP_Melee.Skill Action` (`self.Have Melee`) (- (`local.Skill Num`) 1))))
            (:`2`
              (if (not (`/Game/BP/Melee/BP_Melee.bOnSkill_3 CooldownTime` (`self.Have Melee`)))
                (`/Game/BP/Melee/BP_Melee.Skill Action` (`self.Have Melee`) (- (`local.Skill Num`) 1))))))))))