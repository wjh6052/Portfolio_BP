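; Playable character for the main lobby, with half-scaled move and look input and an interaction prompt.
; On BeginPlay it creates the WB_MainLobby widget, hides the prompt and switches the widget page after a short delay.
; SetInteraction toggles the prompt and adds or clears interactables, and the Interaction input calls Interact on the first one.
; Movement follows control yaw and is gated by status checks, while two test inputs load the demo and lobby maps.
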(event `self.ReceiveBeginPlay`
  (`|ExecutionSequence`
    (:`then_0`
      (bind _returnvalue (`|CreateWidget` "/Game/BP/Widget/WB_MainLobby.WB_MainLobby_C"))
      (bind _output_get (set `self.MainLobbyWidget` _returnvalue))
      (`UserWidget.AddToViewport` _output_get 0)
      (`/Game/BP/Widget/WB_MainLobby.Widget Set Owner` (`self.MainLobbyWidget`) self)
      (`Widget.SetVisibility` (`/Game/BP/Widget/WB_MainLobby.WB_Interaction_Widget` (`self.MainLobbyWidget`)) "Hidden")
      (`KismetSystemLibrary.Delay` 0.2)
      (`self.Set WidgetSwitcher` 1))))

(event `InputAction|Interaction`
  (params (Key :type "Key Structure"))
  (bind _output (`|GetArrayItem` (`self.BP_Interaction`)))
  (:`Pressed`
    (`/Engine/EditorBlueprintResources/StandardMacros.IsValid` _output
      (:`Is Valid`
        (`/Game/BP/Interaction/BP_Interaction.Interact` _output self)))))

(event `InputAction|Test1`
  (params (Key :type "Key Structure"))
  (:`Pressed`
    (`GameplayStatics.OpenLevel` "DemoMap")))

(event `InputAction|test2`
  (params (Key :type "Key Structure"))
  (:`Pressed`
    (`GameplayStatics.OpenLevel` "MainLobby_Map")))

(event `InputAxis|MoveForward`
  (params (AxisValue :type "Float (single-precision)"))
  (bind (_returnvalue_roll _returnvalue_pitch _returnvalue_yaw) (`KismetMathLibrary.BreakRotator` (`self.GetControlRotation`)))
  ;[1 1 1] MoveForward
  (if (!= AxisValue 0.0)
    (set `self.MoveForward` (/ AxisValue 2.0))
    (if (or (`self.Is Status` "NewEnumerator10") (`self.Is Status` "NewEnumerator0"))
      (`self.AddMovementInput` (`KismetMathLibrary.GetForwardVector` (`KismetMathLibrary.MakeRotator` 0.0 0.0 _returnvalue_yaw)) (`self.MoveForward`)))))

(event `InputAxis|MoveRight`
  (params (AxisValue :type "Float (single-precision)"))
  (bind (_returnvalue_roll _returnvalue_pitch _returnvalue_yaw) (`KismetMathLibrary.BreakRotator` (`self.GetControlRotation`)))
  ;[1 1 1] MoveRight
  (if (!= AxisValue 0.0)
    (set `self.MoveRight` (/ AxisValue 2.0))
    (if (or (`self.Is Status` "NewEnumerator10") (`self.Is Status` "NewEnumerator0"))
      (`self.AddMovementInput` (`KismetMathLibrary.GetRightVector` (`KismetMathLibrary.MakeRotator` 0.0 0.0 _returnvalue_yaw)) (`self.MoveRight`)))))

(event `InputAxis|HorizontalLook`
  (params (AxisValue :type "Float (single-precision)"))
  ;[1 1 1] 마우스 회전
  (`self.AddControllerYawInput` (/ AxisValue 2.0)))

(event `InputAxis|VerticalLook`
  (params (AxisValue :type "Float (single-precision)"))
  ;[1 1 1] 마우스 회전
  (`self.AddControllerPitchInput` (/ AxisValue 2.0)))

(fn `Set Interaction`
  (params (On :type Boolean) (`In Interaction` :type "/Game/BP/Interaction/BP_Interaction Object Reference") (`In Text` :type Text))
  (bind _wb_interaction_widget (`/Game/BP/Widget/WB_MainLobby.WB_Interaction_Widget` (`self.MainLobbyWidget`)))
  (if On
    (`Widget.SetVisibility` _wb_interaction_widget "Visible")
    (set `TextBlock.Text` (`local.In Text`) (`/Game/BP/Widget/WB_Interaction_Widget.ObjectNameText` (`/Game/BP/Widget/WB_MainLobby.WB_Interaction_Widget` (`self.MainLobbyWidget`))))
    (set `TextBlock.Text` "F" (`/Game/BP/Widget/WB_Interaction_Widget.InputKeyText` (`/Game/BP/Widget/WB_MainLobby.WB_Interaction_Widget` (`self.MainLobbyWidget`))))
    (`KismetArrayLibrary.Array_AddUnique` (`self.BP_Interaction`) (`local.In Interaction`))
    (else
      (`Widget.SetVisibility` _wb_interaction_widget "Hidden")
      (`KismetArrayLibrary.Array_Clear` (`self.BP_Interaction`)))))

(fn `Set WidgetSwitcher`
  (params (`Switch Num` :type Integer))
  (`WidgetSwitcher.SetActiveWidgetIndex` (`/Game/BP/Widget/WB_MainLobby.WidgetSwitcher` (`self.MainLobbyWidget`)) `Switch Num`))

(fn `UserConstructionScript`
  (`parent.UserConstructionScript`))