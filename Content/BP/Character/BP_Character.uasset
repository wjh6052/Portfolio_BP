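; Character Blueprint providing shared status, movement, damage and ragdoll helpers, likely as a base for game characters.
; Type, status and state live in BPStatusComponent, which receives AnyDamage unless one particular status is active.
; That same status gates Desh, which forwards to the held melee object.
; Damage numbers spawn one Niagara system per digit, offset sideways, yawed by camera control rotation, textured per digit and colored for criticals.
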(event `self.ReceiveBeginPlay`
  (set `/Game/BP/Components/BP_StatusComponent.CharacterType` (`self.CharacterType`) (`self.BP_StatusComponent`)))

(event `self.ReceiveAnyDamage`
  (params (Damage :type "Float (single-precision)") (DamageType :type "DamageType Object Reference") (InstigatedBy :type "Controller Object Reference") (DamageCauser :type "Actor Object Reference"))
  (if (not (`self.Is Status` "NewEnumerator1"))
    (`/Game/BP/Components/BP_StatusComponent.Add Damage` (`self.BP_StatusComponent`) Damage)))

(fn `Desh`
  (if (`self.Is Status` "NewEnumerator1")
    (`/Game/BP/Melee/BP_Melee.Desh` (`/Game/BP/Components/BP_MeleeCompoent.Have Melee` (`self.BP_MeleeCompoent`)))))

(fn `Get CharacterType`
  (returns (CharacterType :type "/Game/BP/Data/Enum/ECharacterType Enum"))
  (return (`/Game/BP/Components/BP_StatusComponent.CharacterType` (`self.BP_StatusComponent`))))

(fn `Get Player State`
  (returns (`Out State` :type "/Game/BP/Data/Enum/EStateType Enum"))
  (return (`/Game/BP/Components/BP_StatusComponent.State Type` (`self.BP_StatusComponent`))))

(fn `Get Status`
  (returns (`Status Type` :type "/Game/BP/Data/Enum/EStatusType Enum"))
  (return (`/Game/BP/Components/BP_StatusComponent.Status Type` (`self.BP_StatusComponent`))))

(fn `Is State`
  (params (NewState :type "/Game/BP/Data/Enum/EStateType Enum" :default "NewEnumerator0"))
  (returns (Result :type Boolean))
  (return (`|EnumEquality` (`/Game/BP/Components/BP_StatusComponent.State Type` (`self.BP_StatusComponent`)) NewState)))

(fn `Is Status`
  (params (`In Status` :type "/Game/BP/Data/Enum/EStatusType Enum" :default "NewEnumerator0"))
  (returns (Result :type Boolean))
  (return (`|EnumEquality` (`/Game/BP/Components/BP_StatusComponent.Status Type` (`self.BP_StatusComponent`)) `In Status`)))

(fn `Make Floating Numbers`
  (params (`In Location` :type "Vector Structure") (`In DamageAmount` :type Integer) (`In On Critical` :type Boolean))
  (locals (`Digit System` :type "NiagaraComponent Object Reference") (`Text Offset` :type "Float (double-precision)" :default 0.0))
  (bind (_returnvalue_roll _returnvalue_pitch _returnvalue_yaw) (`KismetMathLibrary.BreakRotator` (`Controller.GetControlRotation` (`GameplayStatics.GetPlayerController` 0))))
  (for _array_element (`KismetStringLibrary.GetCharacterArrayFromString` (`KismetStringLibrary.Conv_IntToString` `In DamageAmount`))
    (bind _returnvalue (`NiagaraFunctionLibrary.SpawnSystemAtLocation` "/Game/Impact/Damage_Text/NS_Damage_Text.NS_Damage_Text" (`local.In Location`) (`KismetMathLibrary.MakeRotator` 0.0 180.0 _returnvalue_yaw) (0.5 0.5 0.5)))
    (set `local.Digit System` _returnvalue)
    (if (`local.In On Critical`)
      (`FXSystemComponent.SetColorParameter` (`local.Digit System`) "Text Color" (struct :`R` 1.0 :`A` 1.0))
      (else
        (`FXSystemComponent.SetColorParameter` (`local.Digit System`) "Text Color" (struct :`G` 1.0 :`B` 1.0 :`A` 1.0))))
    (`SceneComponent.K2_AddLocalOffset` (`local.Digit System`) (`KismetMathLibrary.MakeVector` 0.0 (`local.Text Offset`)) false false)
    (set `local.Text Offset` (+ (`local.Text Offset`) 25.0))
    (switch `string` _array_element
      (:`0`
        (`NiagaraFunctionLibrary.SetTextureObject` (`local.Digit System`) "user.Digit" "/Game/Impact/Damage_Text/Genshin_font_０.Genshin_font_０"))
      (:`1`
        (`NiagaraFunctionLibrary.SetTextureObject` (`local.Digit System`) "user.Digit" "/Game/Impact/Damage_Text/Genshin_font_１.Genshin_font_１"))
      (:`2`
        (`NiagaraFunctionLibrary.SetTextureObject` (`local.Digit System`) "user.Digit" "/Game/Impact/Damage_Text/Genshin_font_２.Genshin_font_２"))
      (:`3`
        (`NiagaraFunctionLibrary.SetTextureObject` (`local.Digit System`) "user.Digit" "/Game/Impact/Damage_Text/Genshin_font_３.Genshin_font_３"))
      (:`4`
        (`NiagaraFunctionLibrary.SetTextureObject` (`local.Digit System`) "user.Digit" "/Game/Impact/Damage_Text/Genshin_font_４.Genshin_font_４"))
      (:`5`
        (`NiagaraFunctionLibrary.SetTextureObject` (`local.Digit System`) "user.Digit" "/Game/Impact/Damage_Text/Genshin_font_５.Genshin_font_５"))
      (:`6`
        (`NiagaraFunctionLibrary.SetTextureObject` (`local.Digit System`) "user.Digit" "/Game/Impact/Damage_Text/Genshin_font_６.Genshin_font_６"))
      (:`7`
        (`NiagaraFunctionLibrary.SetTextureObject` (`local.Digit System`) "user.Digit" "/Game/Impact/Damage_Text/Genshin_font_７.Genshin_font_７"))
      (:`8`
        (`NiagaraFunctionLibrary.SetTextureObject` (`local.Digit System`) "user.Digit" "/Game/Impact/Damage_Text/Genshin_font_８.Genshin_font_８"))
      (:`9`
        (`NiagaraFunctionLibrary.SetTextureObject` (`local.Digit System`) "user.Digit" "/Game/Impact/Damage_Text/Genshin_font_９.Genshin_font_９")))))

(fn `Ragdoll`
  (set `SkeletalMeshComponent.GlobalAnimRateScale` 0.0 (`self.Mesh`))
  (`PrimitiveComponent.SetSimulatePhysics` (`self.Mesh`) true)
  (`PrimitiveComponent.SetCollisionEnabled` (`self.Mesh`) "QueryAndPhysics")
  (`PrimitiveComponent.SetCollisionEnabled` (`self.CapsuleComponent`) "NoCollision"))

(fn `Set Move`
  (params (CanMove :type Boolean :default false))
  (returns (Result :type Boolean))
  (set `self.bCanMove` CanMove)
  (return false))

(fn `Set State`
  (params (NewState :type "/Game/BP/Data/Enum/EStateType Enum" :default "NewEnumerator0"))
  (returns (Result :type Boolean))
  (set `/Game/BP/Components/BP_StatusComponent.State Type` NewState (`self.BP_StatusComponent`))
  (return false))

(fn `Set Status`
  (params (`New State` :type "/Game/BP/Data/Enum/EStatusType Enum" :default "NewEnumerator0"))
  (returns (Result :type Boolean))
  (set `/Game/BP/Components/BP_StatusComponent.Status Type` `New State` (`self.BP_StatusComponent`))
  (return false))

(fn `Set Walk`
  (params (`In On Walk` :type Boolean))
  (bind _charactermovement (`self.CharacterMovement`))
  (if `In On Walk`
    (set `CharacterMovementComponent.MaxWalkSpeed` 200.0 _charactermovement)
    (else
      (set `CharacterMovementComponent.MaxWalkSpeed` 400.0 _charactermovement))))

(fn `Spawn Damage Text`
  (params (`In Damage` :type "Float (double-precision)") (`In On Critical` :type Boolean))
  (`self.Make Floating Numbers` (`self.K2_GetActorLocation`) (`KismetMathLibrary.FTrunc` `In Damage`) `In On Critical`))

(fn `UserConstructionScript`)