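; BP_Enemy is an enemy character Blueprint with a name and HP display and a target widget that shows when it is selected.
; BeginPlay sets the name from the object name, shows max HP as full and hides the target widget, while AnyDamage refreshes HP text from BPStatusComponent.
; Selection functions toggle the widget, and AttackKnockBack launches the character along a given vector.
; UpdateHPBar is an empty stub.
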(event `self.ReceiveBeginPlay`
  (bind _returnvalue (`KismetStringLibrary.Conv_DoubleToString` (`/Game/BP/Components/BP_StatusComponent.Stat HP Max` (`self.BP_StatusComponent`))))
  (`parent.ReceiveBeginPlay`)
  (`|ExecutionSequence`
    (:`then_0`
      (`TextRenderComponent.K2_SetText` (`self.Actor Name`) (`KismetTextLibrary.Conv_StringToText` (`KismetSystemLibrary.GetObjectName` self)))
      (`TextRenderComponent.K2_SetText` (`self.HP`) (`KismetTextLibrary.Conv_StringToText` (`KismetStringLibrary.Concat_StrStr` _returnvalue " / " _returnvalue))))
    (:`then_3`
      (`self.On Deselected`))))

(event `self.ReceiveTick`
  (params (DeltaSeconds :type "Float (single-precision)")))

(event `self.ReceiveAnyDamage`
  (params (Damage :type "Float (single-precision)") (DamageType :type "DamageType Object Reference") (InstigatedBy :type "Controller Object Reference") (DamageCauser :type "Actor Object Reference"))
  (bind _bp_statuscomponent (`self.BP_StatusComponent`))
  (`parent.ReceiveAnyDamage` Damage DamageType InstigatedBy DamageCauser)
  (`TextRenderComponent.K2_SetText` (`self.HP`) (`KismetTextLibrary.Conv_StringToText` (`KismetStringLibrary.Concat_StrStr` (`KismetStringLibrary.Conv_DoubleToString` (`/Game/BP/Components/BP_StatusComponent.Stat HP` _bp_statuscomponent)) " / " (`KismetStringLibrary.Conv_DoubleToString` (`/Game/BP/Components/BP_StatusComponent.Stat HP Max` _bp_statuscomponent))))))

(fn `Attack Knock Back`
  (params (`In Vector` :type "Vector Structure"))
  (`self.LaunchCharacter` `In Vector` true true))

(fn `On Deselected`
  (`SceneComponent.SetHiddenInGame` (`self.TargetWidget`) true false)
  (return))

(fn `On Selected`
  (`SceneComponent.SetHiddenInGame` (`self.TargetWidget`) false false))

(fn `Update HP Bar`
  (params (`In Top Progress` :type "Float (double-precision)") (`In Delta Seconds` :type "Float (double-precision)")))

(fn `UserConstructionScript`)