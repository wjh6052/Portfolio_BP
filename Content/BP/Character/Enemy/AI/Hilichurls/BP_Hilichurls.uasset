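; Hilichurl enemy Blueprint that adds an animated HP bar and sets a melee weapon shortly after BeginPlay.
; Damage enables per-tick updates of a dynamic material, fed health from the status component.
; Lost health accumulates in a bottom-progress value that drains over time, stopping updates when empty.
; The Desh override destroys the bar and spawns a geometry collection above the actor in its place.
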(event `self.ReceiveBeginPlay`
  (`parent.ReceiveBeginPlay`)
  (`|ExecutionSequence`
    (:`then_0`
      (bind _returnvalue (`KismetMaterialLibrary.CreateDynamicMaterialInstance` "/Game/Object/HP_Bar/MAT_HPBar_Inst.MAT_HPBar_Inst"))
      (bind _output_get (set `self.Dynamic HpBar` _returnvalue))
      (`PrimitiveComponent.SetMaterial` (`self.HPBar`) 1 _output_get)
      (`MaterialInstanceDynamic.SetScalarParameterValue` (`self.Dynamic HpBar`) "TopProgress" 1.0))
    (:`then_1`
      (`KismetSystemLibrary.Delay` 0.5)
      (`/Game/BP/Components/BP_MeleeCompoent.Change Weapon` (`self.BP_MeleeCompoent`) "NewEnumerator12"))))

(event `self.ReceiveTick`
  (params (DeltaSeconds :type "Float (single-precision)"))
  (bind _bp_statuscomponent (`self.BP_StatusComponent`))
  (`parent.ReceiveTick` DeltaSeconds)
  (if (`self.bHpBar`)
    (`self.Update HP Bar` (/ (`/Game/BP/Components/BP_StatusComponent.Stat HP` _bp_statuscomponent) (`/Game/BP/Components/BP_StatusComponent.Stat HP Max` _bp_statuscomponent)) DeltaSeconds)))

(event `self.ReceiveAnyDamage`
  (params (Damage :type "Float (single-precision)") (DamageType :type "DamageType Object Reference") (InstigatedBy :type "Controller Object Reference") (DamageCauser :type "Actor Object Reference"))
  (`parent.ReceiveAnyDamage` Damage DamageType InstigatedBy DamageCauser)
  (set `self.bHpBar` true))

(fn `Desh`
  (`parent.Desh`)
  (`/Engine/EditorBlueprintResources/StandardMacros.IsValid` (`self.HPBar`)
    (:`Is Valid`
      (`ActorComponent.K2_DestroyComponent` (`self.HPBar`))
      (`AddComponent|NODE_AddGeometryCollectionComponent-1` :`RelativeTransform` (`KismetMathLibrary.MakeTransform` (* (`self.GetActorUpVector`) 130) (struct :`Yaw` -90.0))))))

(fn `Update HP Bar`
  (params (`In Top Progress` :type "Float (double-precision)") (`In Delta Seconds` :type "Float (double-precision)"))
  (`parent.Update HP Bar` `In Top Progress` `In Delta Seconds`)
  (set `self.BottomProgress` (+ (`self.BottomProgress`) (* (- (`local.In Top Progress`) (`self.TopProgress`)) -1.0)))
  (set `self.TopProgress` (`local.In Top Progress`))
  (`MaterialInstanceDynamic.SetScalarParameterValue` (`self.Dynamic HpBar`) "TopProgress" (`self.TopProgress`))
  (`MaterialInstanceDynamic.SetScalarParameterValue` (`self.Dynamic HpBar`) "BottomProgress" (`self.BottomProgress`))
  (bind _output_get (set `self.BottomProgress` (`KismetMathLibrary.FClamp` (- (`self.BottomProgress`) (* (`local.In Delta Seconds`) (`self.HPBar Speed`))) 0.0 (`self.BottomProgress`))))
  (if (<= _output_get 0.0)
    (set `self.bHpBar` false)))

(fn `UserConstructionScript`
  (`parent.UserConstructionScript`))