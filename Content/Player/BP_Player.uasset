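; Player character Blueprint handling walk and run speeds, mouse look, spring-arm zoom, jumping, climbing and flight.
; Movement and jump inputs are gated by CanMove and switch on StatusType between control-yaw movement and the climbing component.
; Jump also starts flight when falling or stops it when flying, through the flight component.
; Dash and RunToStop push the actor forward with swept timeline lerps, and hidden wings spawned at BeginPlay attach on a test input.
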(event `self.ReceiveBeginPlay`
  (bind _returnvalue (`|SpawnActorFromClass` "/Game/Player/BP_Wings.BP_Wings_C" (`KismetMathLibrary.MakeTransform` (0.0 0.0 0.0)) "Undefined" "MultiplyWithRoot" self null))
  (bind _output_get (set `self.Wings` _returnvalue))
  (`self.SetActorHiddenInGame` _output_get true))

(event `InputAction|Tast`
  (params (Key :type "Key Structure"))
  (:`Pressed`
    (`self.SetActorHiddenInGame` (`self.Wings`) false)
    (`self.K2_AttachToComponent` (`self.Wings`) (`self.Mesh`) "Wings" "KeepRelative" "KeepRelative" "KeepRelative" true)))

(event `InputAction|Run`
  (params (Key :type "Key Structure"))
  (bind _charactermovement (`self.CharacterMovement`))
  ;[1 1 1] 달리기
  (:`Pressed`
    (set `CharacterMovementComponent.MaxWalkSpeed` 600.0 _charactermovement))
  (:`Released`
    (set `CharacterMovementComponent.MaxWalkSpeed` 400.0 _charactermovement)))

(event `InputAction|Walk`
  (params (Key :type "Key Structure"))
  (bind _charactermovement (`self.CharacterMovement`))
  ;[1 1 1] 걷기
  (:`Pressed`
    (set `CharacterMovementComponent.MaxWalkSpeed` 200.0 _charactermovement))
  (:`Released`
    (set `CharacterMovementComponent.MaxWalkSpeed` 400.0 _charactermovement)))

(event `InputAxis|MoveForward`
  (params (AxisValue :type "Float (single-precision)"))
  (bind (_returnvalue_roll _returnvalue_pitch _returnvalue_yaw) (`KismetMathLibrary.BreakRotator` (`self.GetControlRotation`)))
  (bind _output_get (set `self.MoveForward` AxisValue))
  (if (!= _output_get 0.0)
    (if (`self.bCanMove`)
      (switch `/Game/Data/Enum/EStatusType` (`self.StatusType`)
        (:`NewEnumerator0`
          (`self.AddMovementInput` (`KismetMathLibrary.GetForwardVector` (`KismetMathLibrary.MakeRotator` 0.0 0.0 _returnvalue_yaw)) (`self.MoveForward`)))
        (:`NewEnumerator1`
          (`/Game/Components/BP_ClimbingComponent.ClimbingMove` (`self.BP_ClimbingComponent`) (`self.GetActorUpVector`) (`self.MoveForward`) false))))))

(event `InputAxis|MoveRight`
  (params (AxisValue :type "Float (single-precision)"))
  (bind (_returnvalue_roll _returnvalue_pitch _returnvalue_yaw) (`KismetMathLibrary.BreakRotator` (`self.GetControlRotation`)))
  (bind _output_get (set `self.MoveRight` AxisValue))
  (if (!= _output_get 0.0)
    (if (`self.bCanMove`)
      (switch `/Game/Data/Enum/EStatusType` (`self.StatusType`)
        (:`NewEnumerator0`
          (`self.AddMovementInput` (`KismetMathLibrary.GetRightVector` (`KismetMathLibrary.MakeRotator` 0.0 0.0 _returnvalue_yaw)) (`self.MoveRight`)))
        (:`NewEnumerator1`
          (`/Game/Components/BP_ClimbingComponent.ClimbingMove` (`self.BP_ClimbingComponent`) (`self.GetActorRightVector`) (`self.MoveRight`) true))))))

(event `InputAction|Jump`
  (params (Key :type "Key Structure"))
  (bind _bcanmove (`self.bCanMove`))
  (:`Pressed`
    (if _bcanmove
      (switch `/Game/Data/Enum/EStatusType` (`self.StatusType`)
        (:`NewEnumerator0`
          (`self.Jump`)
          (`/Game/Components/BP_ClimbingComponent.CheckClimbing` (`self.BP_ClimbingComponent`))
          (if (`self.IsMovement Mode` "MOVE_Falling")
            (`/Game/Components/BP_FlightComponent.StartFlight` (`self.BP_FlightComponent`))
            (elif (`self.IsMovement Mode` "MOVE_Flying")
              (`/Game/Components/BP_FlightComponent.StopFlight` (`self.BP_FlightComponent`)))))
        (:`NewEnumerator1`
          (`/Game/Components/BP_ClimbingComponent.Climbing_End` (`self.BP_ClimbingComponent`))))))
  (:`Released`
    (if _bcanmove
      (`self.StopJumping`))))

(event `InputAxis|HorizontalLook`
  (params (AxisValue :type "Float (single-precision)"))
  ;[1 1 1] 마우스 회전
  (`self.AddControllerYawInput` AxisValue))

(event `InputAxis|VerticalLook`
  (params (AxisValue :type "Float (single-precision)"))
  ;[1 1 1] 마우스 회전
  (`self.AddControllerPitchInput` AxisValue))

(event `InputAxis|CameraZoom`
  (params (AxisValue :type "Float (single-precision)"))
  (bind _springarm (`self.SpringArm`))
  ;[1 1 1] 마우스 휠
  (set `SpringArmComponent.TargetArmLength` (`KismetMathLibrary.FClamp` (+ (* AxisValue 10.0) (`SpringArmComponent.TargetArmLength` _springarm)) 150.0 1000.0) _springarm))

(event `self.ReceiveTick`
  (params (DeltaSeconds :type "Float (single-precision)")))

(event `Dash`
  ;[1 1 1] 대쉬
  (bind _output_get (set `self.StartPoint` (`self.K2_GetActorLocation`)))
  (set `self.EndPoint` (+ _output_get (* (`self.GetActorForwardVector`) 450.0)))
  (`self.PlayAnimMontage` "/Game/Animation/Unarmed/Dash1_Montage.Dash1_Montage")
  (bind (_direction _output) (`Timeline|Dash_Timeline` :!via `PlayFromStart`)
    (:`Update`
      (`self.K2_SetActorLocation` (`KismetMathLibrary.VLerp` (`self.StartPoint`) (`self.EndPoint`) _output) true))))

(event `Run To Stop`
  ;[1 1 1] 뛰다가 멈추기
  (bind _output_get (set `self.StartPoint` (`self.K2_GetActorLocation`)))
  (set `self.EndPoint` (+ _output_get (* (`self.GetActorForwardVector`) 50.0)))
  (bind (_direction _out_put) (`Timeline|RunToStop_Timeline` :!via `PlayFromStart`)
    (:`Update`
      (`self.K2_SetActorLocation` (`KismetMathLibrary.VLerp` (`self.StartPoint`) (`self.EndPoint`) _out_put) true))))

(fn `IsMovement Mode`
  (params (`Movement Mode` :type "EMovementMode Enum" :default "MOVE_None"))
  (returns (ReturnValue :type Boolean))
  (return (`|EnumEquality` `Movement Mode` (`CharacterMovementComponent.MovementMode` (`self.CharacterMovement`)))))

(fn `UserConstructionScript`)