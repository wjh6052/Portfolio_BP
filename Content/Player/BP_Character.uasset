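; Player character Blueprint that holds the character's state, status and movement-permission values.
; IsState and IsStatus compare a given value against StateType and StatusType.
; SetState, SetStatus and SetMove overwrite StateType, StatusType and CanMove with no transition checks, each returning false.
; The construction script is empty, and the file shows no input, movement or event logic.
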(fn `IsState`
  (params (NewState :type "/Game/Data/Enum/EStateType Enum" :default "NewEnumerator0"))
  (returns (Result :type Boolean))
  (return (`|EnumEquality` (`self.StateType`) NewState)))

(fn `IsStatus`
  (params (NewStaus :type "/Game/Data/Enum/EStatusType Enum" :default "NewEnumerator0"))
  (returns (Result :type Boolean))
  (return (`|EnumEquality` (`self.StatusType`) NewStaus)))

(fn `SetMove`
  (params (CanMove :type Boolean))
  (returns (Result :type Boolean))
  (set `self.bCanMove` CanMove)
  (return false))

(fn `SetState`
  (params (NewState :type "/Game/Data/Enum/EStateType Enum" :default "NewEnumerator0"))
  (returns (Result :type Boolean))
  (set `self.StateType` NewState)
  (return false))

(fn `SetStatus`
  (params (NewStaus :type "/Game/Data/Enum/EStatusType Enum" :default "NewEnumerator0"))
  (returns (Result :type Boolean))
  (set `self.StatusType` NewStaus)
  (return false))

(fn `UserConstructionScript`)